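; BP_CatPlayerController is a player controller that runs a post-process fade-out before travelling to the ChristmasMarket3 level.
; Its SetMaterial event creates a dynamic fade material and adds it as a blendable to the S_VRPawnTest player's camera.
; A timeline drives the material's FadeAmount parameter, then opens the level when finished.
; BeginPlay, Tick and the SetMat function are empty, and SetMaterial has no caller in this graph.
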(event `SetMaterial`
  (bind _ass_vrpawn_test (cast `/Game/VRTemplate/Blueprints/S_VRPawnTest` (`GameplayStatics.GetPlayerCharacter` 0)))
  (bind _returnvalue (`KismetMaterialLibrary.CreateDynamicMaterialInstance` "/Game/LCU/FadeOutMat_Inst.FadeOutMat_Inst"))
  (set `self.Mat` _returnvalue)
  (`CameraComponent.AddOrUpdateBlendable` (`/Game/VRTemplate/Blueprints/S_VRPawnTest.Camera` _ass_vrpawn_test) _returnvalue 1.0)
  (bind (_direction _amount) (`Timeline|FadeAmount`)
    (:`Update`
      (`MaterialInstanceDynamic.SetScalarParameterValue` (`self.Mat`) "FadeAmount" _amount))
    (:`Finished`
      (`GameplayStatics.OpenLevel` "ChristmasMarket3"))))

(fn `SetMat`)

(fn `UserConstructionScript`)