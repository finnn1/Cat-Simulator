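; BP_TutoTriggerBox is a trigger box that reveals tutorial actors: left controller, right controller and tutorial widget sets.
; The reveal runs when the player character begins overlapping the box, or at BeginPlay if RenderBegin is set.
; VisiblaActors makes one PrimitiveComponent per listed actor visible, without propagating to children.
; Nothing in the blueprint hides them again.
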(event `self.ReceiveBeginPlay`
  (if (`self.bRenderBegin`)
    (`self.VisiblaActors` (`self.ControllerLeft`))
    (`self.VisiblaActors` (`self.TutoWidget`))
    (`self.VisiblaActors` (`self.ControllerRight`))))

(event `self.Box.OnComponentBeginOverlap`
  (params (OverlappedComponent :type "PrimitiveComponent Object Reference") (OtherActor :type "Actor Object Reference") (OtherComp :type "PrimitiveComponent Object Reference") (OtherBodyIndex :type Integer) (bFromSweep :type Boolean) (SweepResult :type "HitResult Structure (by ref)"))
  (if (== OtherActor (`GameplayStatics.GetPlayerCharacter` 0))
    (`self.VisiblaActors` (`self.ControllerLeft`))
    (`self.VisiblaActors` (`self.TutoWidget`))
    (`self.VisiblaActors` (`self.ControllerRight`))))

(fn `UserConstructionScript`)

(fn `VisiblaActors`
  (params (Actors :type "Array of Actor Object Reference"))
  (if (`KismetArrayLibrary.Array_IsEmpty` Actors)
    (return)
    (else
      (for _array_element Actors
        (`SceneComponent.SetVisibility` (`self.GetComponentByClass` _array_element "/Script/Engine.PrimitiveComponent") true false))
      (return))))