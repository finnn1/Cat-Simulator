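; BP_Meat is a grillable meat food item with a timer widget, grilling sound and smoke.
; StartGrilling fades in the sound, restarts and shows the five-second timer, then plays one of two timelines based on Fliped.
; The unflipped timeline activates smoke when it finishes.
; A mesh hit destroys the meat once it is flipped and the timer is ready; the Filp event is an empty stub.
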(event `self.ReceiveBeginPlay`
  (`parent.ReceiveBeginPlay`)
  (bind _aswbp_timer (cast `/Game/DynamicCookingSystem/Widgets/Timer/WBP_Timer` (`WidgetComponent.GetUserWidgetObject` (`self.TimerWidget`))))
  (bind _output_get (set `self.WBP Timer` _aswbp_timer))
  (`Widget.SetVisibility` _output_get "Hidden"))

(event `StartGrilling`
  (bind _wbp_timer (`self.WBP Timer`))
  (`AudioComponent.FadeIn` (`self.GrillingSound`) 0.1 1.0 0.0 "Linear")
  (`/Game/DynamicCookingSystem/Widgets/Timer/WBP_Timer.ResetTimer` _wbp_timer)
  (`Widget.SetVisibility` _wbp_timer "Visible")
  (`/Game/DynamicCookingSystem/Widgets/Timer/WBP_Timer.StartTimer` _wbp_timer 5.0)
  (if (`self.Fliped`)
    (`Timeline|Timeline`)
    (else
      (`Timeline|GrillTimeline`
        (:`Finished`
          (`ActorComponent.Activate` (`self.Smoke`) false))))))

(event `self.StaticMeshComponent.OnComponentHit`
  (params (HitComponent :type "PrimitiveComponent Object Reference") (OtherActor :type "Actor Object Reference") (OtherComp :type "PrimitiveComponent Object Reference") (NormalImpulse :type "Vector Structure") (Hit :type "HitResult Structure (by ref)"))
  (if (`/Game/DynamicCookingSystem/Widgets/Timer/WBP_Timer.Ready` (`self.WBP Timer`))
    (if (`self.Fliped`)
      (`self.K2_DestroyActor`))))

(event `Filp`)

(fn `UserConstructionScript`
  (`parent.UserConstructionScript`))