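; BP_Knife is a knife item that cuts food items it hits into sliced pieces.
; When its static mesh hits a BP_FoodItem, it looks up the food's data table row through its ItemDataComponent and checks for the CUT property.
; Cuttable food is destroyed after spawning its configured number of SlicedFood actors slightly above its location, regardless of collisions.
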(event `self.StaticMeshComponent.OnComponentHit`
  (params (HitComponent :type "PrimitiveComponent Object Reference") (OtherActor :type "Actor Object Reference") (OtherComp :type "PrimitiveComponent Object Reference") (NormalImpulse :type "Vector Structure") (Hit :type "HitResult Structure (by ref)"))
  (bind (_asbp_food_item _bsuccess) (cast `/Game/LCU/Item/BP_FoodItem` OtherActor :!pure true))
  (bind (_returnvalue_x _returnvalue_y _returnvalue_z) (`KismetMathLibrary.BreakVector` (`self.K2_GetActorLocation` _asbp_food_item)))
  (bind (_itemid_datatable _itemid_rowname) (break `DataTableRowHandle` (`UItemDataComponent.ItemID` (`UItem.ItemDataComponent` _asbp_food_item))))
  (if _bsuccess
    (bind _returnvalue (`|GetDataTableRow` _itemid_datatable _itemid_rowname)
      (:`then`
        (if (`.ReturnValue` (`BlueprintMapLibrary.Map_Find` (`.ItemProperty` (break `ItemStruct` _returnvalue)) "CUT"))
          (for _ (range (`UFoodItem.SliceNum` _asbp_food_item))
            (`|SpawnActorFromClass` (`UFoodItem.SlicedFood` _asbp_food_item) (`KismetMathLibrary.MakeTransform` (`KismetMathLibrary.MakeVector` _returnvalue_x _returnvalue_y (+ _returnvalue_z 10.0))) "AlwaysSpawn" "MultiplyWithRoot" null null))
          (`self.K2_DestroyActor` _asbp_food_item))))))

(fn `UserConstructionScript`
  (`parent.UserConstructionScript`))