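; Grill appliance for the cooking station, switched on and off by a clickable button that only responds in Grilling mode and shows an On/Off hover widget.
; Toggling drives sound, indicator light, button position and a heat-plate material timeline, whose completion toggles haze and starts grilling waiting items when on.
; Two placement overlaps register BP_MixedActor food and track slot occupancy, grilling it immediately if running.
; Interact hands off to the station's StartCooking.
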(event `self.OnButton.OnClicked`
  (params (TouchedComponent :type "PrimitiveComponent Object Reference") (ButtonPressed :type "Key Structure"))
  (switch `/Game/DynamicCookingSystem/Data/E_CookingMode` (`/Game/DynamicCookingSystem/Blueprints/BP_CookingStation.CookingMode` (`self.CookingStationRef`))
    (:`NewEnumerator3`
      (`self.RunGrill`))))

(event `RunGrill`
  (bind _light (`self.Light`))
  (bind _onbutton (`self.OnButton`))
  (bind _n_haze (`self.N_Haze`))
  (bind _actorstogrill (`self.ActorsToGrill`))
  (bind _grillsound (`self.GrillSound`))
  (`GameplayStatics.PlaySound2D` "/Engine/VREditor/Sounds/UI/Flashlight_Switch.Flashlight_Switch" 1.0 1.0 0.0 null null)
  (if (`self.IsRunning`)
    (bind _output_get (set `self.IsRunning` false))
    (`/Game/DynamicCookingSystem/Widgets/WBP_CookingUINameWidget.SetWidget` (`self.UINameWidget`) _output_get)
    (`AudioComponent.FadeOut` _grillsound 0.5 0.0 "Linear")
    (`MeshComponent.SetScalarParameterValueOnMaterials` _light "OnLight" 0.0)
    (`SceneComponent.K2_SetRelativeLocation` _onbutton (-2.0 16.0 4.0) true false)
    (bind (_direction _newtrack_0) (`Timeline|HeatTimeline` :!via `Reverse` :!label _label)
      (:`Update`
        (`MeshComponent.SetScalarParameterValueOnMaterials` (`self.HeatPlate`) "Alpha" _newtrack_0))
      (:`Finished`
        (if (`self.IsRunning`)
          (`ActorComponent.Activate` _n_haze false)
          (if (not (`KismetArrayLibrary.Array_IsEmpty` _actorstogrill))
            (for _array_element _actorstogrill
              (bind _wbp_timer (`/Game/DynamicCookingSystem/Blueprints/ParentActors/BP_MixedActor.WBP Timer` _array_element))
              (if (`/Game/DynamicCookingSystem/Widgets/Timer/WBP_Timer.InProgress` _wbp_timer)
                _
                (elif (not (`/Game/DynamicCookingSystem/Widgets/Timer/WBP_Timer.Ready` _wbp_timer))
                  (`/Game/DynamicCookingSystem/Blueprints/ParentActors/BP_MixedActor.StartGrilling` _array_element)))))
          (else
            (`ActorComponent.Deactivate` _n_haze)))))
    (else
      (bind _output_get_2 (set `self.IsRunning` true))
      (`/Game/DynamicCookingSystem/Widgets/WBP_CookingUINameWidget.SetWidget` (`self.UINameWidget`) _output_get_2)
      (`AudioComponent.FadeIn` _grillsound 0.5 1.0 0.0 "Linear")
      (`MeshComponent.SetScalarParameterValueOnMaterials` _light "OnLight" 10.0)
      (`SceneComponent.K2_SetRelativeLocation` _onbutton (-2.0 14.0 4.0) true false)
      (goto _label))))

(event `self.OnButton.OnBeginCursorOver`
  (params (TouchedComponent :type "PrimitiveComponent Object Reference"))
  (switch `/Game/DynamicCookingSystem/Data/E_CookingMode` (`/Game/DynamicCookingSystem/Blueprints/BP_CookingStation.CookingMode` (`self.CookingStationRef`))
    (:`NewEnumerator3`
      (bind _returnvalue (`|CreateWidget` "/Game/DynamicCookingSystem/Widgets/WBP_CookingUINameWidget.WBP_CookingUINameWidget_C" null "Off" "On"))
      (bind _output_get (set `self.UINameWidget` _returnvalue))
      (`UserWidget.AddToViewport` _output_get 0)
      (`/Game/DynamicCookingSystem/Widgets/WBP_CookingUINameWidget.SetWidget` _output_get (`self.IsRunning`)))))

(event `self.OnButton.OnEndCursorOver`
  (params (TouchedComponent :type "PrimitiveComponent Object Reference"))
  (switch `/Game/DynamicCookingSystem/Data/E_CookingMode` (`/Game/DynamicCookingSystem/Blueprints/BP_CookingStation.CookingMode` (`self.CookingStationRef`))
    (:`NewEnumerator3`
      (`Widget.RemoveFromParent` (`self.UINameWidget`)))))

(event `self.GrillPlace.OnComponentBeginOverlap`
  (params (OverlappedComponent :type "PrimitiveComponent Object Reference") (OtherActor :type "Actor Object Reference") (OtherComp :type "PrimitiveComponent Object Reference") (OtherBodyIndex :type Integer) (bFromSweep :type Boolean) (SweepResult :type "HitResult Structure (by ref)"))
  (bind _asbp_mixed_actor (cast `/Game/DynamicCookingSystem/Blueprints/ParentActors/BP_MixedActor` OtherActor))
  (set `/Game/DynamicCookingSystem/Blueprints/ParentActors/BP_MixedActor.CookingStation` (`self.CookingStationRef`) _asbp_mixed_actor)
  (set `self.FirstSpanwerInUse` true)
  (set `/Game/DynamicCookingSystem/Blueprints/ParentActors/BP_MixedActor.OnGrill` true _asbp_mixed_actor)
  (`KismetArrayLibrary.Array_Add` (`self.ActorsToGrill`) _asbp_mixed_actor)
  (if (`self.IsRunning`)
    (bind _wbp_timer (`/Game/DynamicCookingSystem/Blueprints/ParentActors/BP_MixedActor.WBP Timer` _asbp_mixed_actor))
    (if (`/Game/DynamicCookingSystem/Widgets/Timer/WBP_Timer.InProgress` _wbp_timer)
      _
      (elif (not (`/Game/DynamicCookingSystem/Widgets/Timer/WBP_Timer.Ready` _wbp_timer))
        (`/Game/DynamicCookingSystem/Blueprints/ParentActors/BP_MixedActor.StartGrilling` _asbp_mixed_actor)))))

(event `self.GrillPlace.OnComponentEndOverlap`
  (params (OverlappedComponent :type "PrimitiveComponent Object Reference") (OtherActor :type "Actor Object Reference") (OtherComp :type "PrimitiveComponent Object Reference") (OtherBodyIndex :type Integer))
  (bind _asbp_mixed_actor (cast `/Game/DynamicCookingSystem/Blueprints/ParentActors/BP_MixedActor` OtherActor))
  (set `self.FirstSpanwerInUse` false)
  (`KismetArrayLibrary.Array_RemoveItem` (`self.ActorsToGrill`) _asbp_mixed_actor)
  (set `/Game/DynamicCookingSystem/Blueprints/ParentActors/BP_MixedActor.OnGrill` false _asbp_mixed_actor))

(event `self.GrillPlace2.OnComponentBeginOverlap`
  (params (OverlappedComponent :type "PrimitiveComponent Object Reference") (OtherActor :type "Actor Object Reference") (OtherComp :type "PrimitiveComponent Object Reference") (OtherBodyIndex :type Integer) (bFromSweep :type Boolean) (SweepResult :type "HitResult Structure (by ref)"))
  (bind _asbp_mixed_actor (cast `/Game/DynamicCookingSystem/Blueprints/ParentActors/BP_MixedActor` OtherActor))
  (set `/Game/DynamicCookingSystem/Blueprints/ParentActors/BP_MixedActor.CookingStation` (`self.CookingStationRef`) _asbp_mixed_actor)
  (set `self.SecondSpanwerInUse` true)
  (set `/Game/DynamicCookingSystem/Blueprints/ParentActors/BP_MixedActor.OnGrill` true _asbp_mixed_actor)
  (`KismetArrayLibrary.Array_Add` (`self.ActorsToGrill`) _asbp_mixed_actor)
  (if (`self.IsRunning`)
    (bind _wbp_timer (`/Game/DynamicCookingSystem/Blueprints/ParentActors/BP_MixedActor.WBP Timer` _asbp_mixed_actor))
    (if (`/Game/DynamicCookingSystem/Widgets/Timer/WBP_Timer.InProgress` _wbp_timer)
      _
      (elif (not (`/Game/DynamicCookingSystem/Widgets/Timer/WBP_Timer.Ready` _wbp_timer))
        (`/Game/DynamicCookingSystem/Blueprints/ParentActors/BP_MixedActor.StartGrilling` _asbp_mixed_actor)))))

(event `self.GrillPlace2.OnComponentEndOverlap`
  (params (OverlappedComponent :type "PrimitiveComponent Object Reference") (OtherActor :type "Actor Object Reference") (OtherComp :type "PrimitiveComponent Object Reference") (OtherBodyIndex :type Integer))
  (bind _asbp_mixed_actor (cast `/Game/DynamicCookingSystem/Blueprints/ParentActors/BP_MixedActor` OtherActor))
  (set `self.SecondSpanwerInUse` false)
  (`KismetArrayLibrary.Array_RemoveItem` (`self.ActorsToGrill`) _asbp_mixed_actor)
  (set `/Game/DynamicCookingSystem/Blueprints/ParentActors/BP_MixedActor.OnGrill` false _asbp_mixed_actor))

(event `/Game/DynamicCookingSystem/Blueprints/Interface/BI_Interact.Interact`
  (`/Game/DynamicCookingSystem/Blueprints/BP_CookingStation.StartCooking` (`self.CookingStationRef`)))

(fn `UserConstructionScript`)