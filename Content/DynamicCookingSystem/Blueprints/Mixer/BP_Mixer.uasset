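; Interactive mixer for the cooking system, with clickable power and lid buttons that respond in the station's Mixing mode.
; An overlap box collects food chunks and samples three colours when the third arrives.
; Running spins the blade and shakes the bowl; a closed lid turns chunks into a tinted BP_MixedActor and starts a timer, while an open lid destroys them with effects.
; RemoveChunks returns items to the player's inventory.
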(event `self.ReceiveBeginPlay`
  (bind _aswbp_mixer_screen (cast `/Game/DynamicCookingSystem/Widgets/WBP_MixerScreen` (`WidgetComponent.GetUserWidgetObject` (`self.MixerScreen`))))
  (bind _output_get (set `self.Mixer Screen Widget` _aswbp_mixer_screen))
  (set `/Game/DynamicCookingSystem/Widgets/WBP_MixerScreen.MixerRef` self _output_get)
  (`MovementComponent.SetUpdatedComponent` (`self.RotatingMovement`) (`self.SpinnerBlade`))
  (bind _aswbp_timer (cast `/Game/DynamicCookingSystem/Widgets/Timer/WBP_Timer` (`WidgetComponent.GetUserWidgetObject` (`self.TimerWidget`))))
  (bind _output_get_2 (set `self.WBP Timer` _aswbp_timer))
  (set `/Game/DynamicCookingSystem/Widgets/Timer/WBP_Timer.CookingStationRef` (`self.CookingStationRef`) _output_get_2)
  (`Widget.SetVisibility` _output_get_2 "Hidden"))

(event `OpenLid`
  (`/Game/DynamicCookingSystem/Widgets/Timer/WBP_Timer.ResetTimer` (`self.WBP Timer`))
  (if (`self.OpeningInProgress`)
    _
    (elif (not (`self.IsRunning`))
      (`GameplayStatics.PlaySound2D` "/Engine/VREditor/Sounds/UI/Flashlight_Switch.Flashlight_Switch" 1.0 1.0 0.0 null null)
      (if (`self.LidOpen`)
        (`SceneComponent.K2_SetRelativeLocation` (`self.OpenLidButton`) (-9.0 16.0 4.0) true false)
        (bind (_direction _alpha) (`Timeline|OpeningLid` :!via `Reverse` :!label _label)
          (:`Update`
            (set `self.OpeningInProgress` true)
            (`SceneComponent.K2_SetRelativeLocationAndRotation` (`self.Lid`) (`KismetMathLibrary.VLerp` (0.294975 -0.349754 -0.262215) (0.294975 -58.0 31.62405) _alpha) (`KismetMathLibrary.RLerp` (struct) (struct :`Roll` -100.0) _alpha) true false))
          (:`Finished`
            (set `self.OpeningInProgress` false)
            (if (`self.LidOpen`)
              (bind _output_get (set `self.LidOpen` false))
              (`/Game/DynamicCookingSystem/Widgets/WBP_CookingUINameWidget.SetWidget` (`self.UINameWidget`) _output_get)
              (else
                (bind _output_get_2 (set `self.LidOpen` true))
                (`/Game/DynamicCookingSystem/Widgets/WBP_CookingUINameWidget.SetWidget` (`self.UINameWidget`) _output_get_2)))))
        (else
          (`SceneComponent.K2_SetRelativeLocation` (`self.OpenLidButton`) (-9.0 14.0 4.0) true false)
          (goto _label))))))

(event `Shake`
  (bind (_direction _time) (`Timeline|ShakeTimeline` :!via `PlayFromStart`)
    (:`Update`
      (`SceneComponent.K2_SetRelativeLocation` (`self.Bowl`) (`KismetMathLibrary.VLerp` (-0.5 0.0 46.0) (0.5 0.0 46.0) _time) true false))
    (:`Finished`
      (`TimelineComponent.PlayFromStart` (`self.ShakeTimeline`)))))

(event `EndShake`
  (`TimelineComponent.Stop` (`self.ShakeTimeline`))
  (`SceneComponent.K2_SetRelativeLocation` (`self.Bowl`) (0.0 0.0 46.0) true false))

(event `RunMixer`
  (bind _mixersound (`self.MixerSound`))
  (bind _onbutton (`self.OnButton`))
  (bind _light (`self.Light`))
  (bind _wbp_timer (`self.WBP Timer`))
  (`GameplayStatics.PlaySound2D` "/Engine/VREditor/Sounds/UI/Flashlight_Switch.Flashlight_Switch" 1.0 1.0 0.0 null null)
  (if (`self.IsRunning`)
    (bind _output_get (set `self.IsRunning` false))
    (`self.EndShake`)
    (`/Game/DynamicCookingSystem/Widgets/WBP_CookingUINameWidget.SetWidget` (`self.UINameWidget`) _output_get)
    (`AudioComponent.FadeOut` _mixersound 0.1 0.0 "Linear")
    (`SceneComponent.K2_SetRelativeLocation` _onbutton (-2.0 16.0 4.0) true false)
    (`MeshComponent.SetScalarParameterValueOnMaterials` _light "OnLight" 0.0)
    (set `RotatingMovementComponent.RotationRate` (struct) (`self.RotatingMovement`))
    (else
      (`/Engine/EditorBlueprintResources/StandardMacros.IsValid` (`self.MixedActor`)
        (:`Is Not Valid`
          (bind _output_get_2 (set `self.IsRunning` true))
          (`self.Shake`)
          (`/Game/DynamicCookingSystem/Widgets/WBP_CookingUINameWidget.SetWidget` (`self.UINameWidget`) _output_get_2)
          (`AudioComponent.FadeIn` _mixersound 0.1 1.0 0.0 "Linear")
          (`SceneComponent.K2_SetRelativeLocation` _onbutton (-2.0 14.0 4.0) true false)
          (`MeshComponent.SetScalarParameterValueOnMaterials` _light "OnLight" 10.0)
          (set `RotatingMovementComponent.RotationRate` (struct :`Yaw` 1000.0) (`self.RotatingMovement`))
          (if (not (`KismetArrayLibrary.Array_IsEmpty` (`self.ChunksInTheMixer`)))
            (for _array_element (`self.ChunksInTheMixer`)
              (if (`self.LidOpen`)
                (`/Game/DynamicCookingSystem/Blueprints/ParentActors/BP_Chunk.MixFX` _array_element)
                (`self.K2_DestroyActor` _array_element)
                (else
                  (`self.K2_DestroyActor` _array_element)
                  (`Widget.SetVisibility` _wbp_timer "Visible")
                  (`/Game/DynamicCookingSystem/Widgets/Timer/WBP_Timer.StartTimer` _wbp_timer 5.0))))
            (`KismetArrayLibrary.Array_Clear` (`self.ChunksInTheMixer`))
            ;[1 1 1] Add Materials from chunks
            (if (not (`self.LidOpen`))
              (bind _returnvalue (`|SpawnActorFromClass` "/Game/DynamicCookingSystem/Blueprints/ParentActors/BP_MixedActor.BP_MixedActor_C" (`KismetMathLibrary.MakeTransform` (`SceneComponent.K2_GetComponentLocation` (`self.MixedActorSpawner`))) "Undefined" "OverrideRootScale" null null))
              (set `/Game/DynamicCookingSystem/Blueprints/ParentActors/BP_MixedActor.CookingStation` (`self.CookingStationRef`) _returnvalue)
              (set `self.MixedActor` _returnvalue)
              (`/Game/DynamicCookingSystem/Blueprints/ParentActors/BP_MixedActor.SetMaterial` _returnvalue (`self.Color1`) (`self.Color2`) (`self.Color3`)))))))))

(event `self.OnButton.OnClicked`
  (params (TouchedComponent :type "PrimitiveComponent Object Reference") (ButtonPressed :type "Key Structure"))
  (switch `/Game/DynamicCookingSystem/Data/E_CookingMode` (`/Game/DynamicCookingSystem/Blueprints/BP_CookingStation.CookingMode` (`self.CookingStationRef`))
    (:`NewEnumerator2`
      (if (not (`/Game/DynamicCookingSystem/Widgets/Timer/WBP_Timer.InProgress` (`self.WBP Timer`)))
        (`self.RunMixer`)))))

(event `self.OpenLidButton.OnClicked`
  (params (TouchedComponent :type "PrimitiveComponent Object Reference") (ButtonPressed :type "Key Structure"))
  (switch `/Game/DynamicCookingSystem/Data/E_CookingMode` (`/Game/DynamicCookingSystem/Blueprints/BP_CookingStation.CookingMode` (`self.CookingStationRef`))
    (:`NewEnumerator2`
      (if (not (`/Game/DynamicCookingSystem/Widgets/Timer/WBP_Timer.InProgress` (`self.WBP Timer`)))
        (`self.OpenLid`)))))

(event `RemoveChunks`
  (bind _inventorycomponent (message `/Game/DynamicCookingSystem/Blueprints/Interface/BI_GetData.GetInventory` (`GameplayStatics.GetPlayerCharacter` 0)))
  (if (== (`/Game/DynamicCookingSystem/Blueprints/BP_CookingStation.LastAmount` (`self.CookingStationRef`)) 0)
    (for _array_element (`self.ChunksInTheMixer`)
      (`/Game/DynamicCookingSystem/Blueprints/CookingInventory/AC_CookingInventory.AddToInventory` _inventorycomponent (make `/Game/DynamicCookingSystem/Blueprints/CookingInventory/F_InventorySlotStruct` (`/Game/DynamicCookingSystem/Blueprints/ParentActors/BP_Chunk.Item Details Struct` _array_element) 1))
      (`self.K2_DestroyActor` _array_element))
    (`KismetArrayLibrary.Array_Clear` (`self.ChunksInTheMixer`))
    (else
      (for _array_element_2 (`self.ChunksInTheMixer`)
        (bind _itemdetails (break `/Game/DynamicCookingSystem/Blueprints/CookingInventory/F_InventorySlotStruct` (`|GetArrayItem` (`/Game/DynamicCookingSystem/Blueprints/CookingInventory/AC_CookingInventory.Inventory` _inventorycomponent) (`/Game/DynamicCookingSystem/Blueprints/ParentActors/BP_Chunk.Index` _array_element_2))))
        (if (`|EnumEquality` (`.FoodType_20_EA19BE294A20745246A9128CC537F1CF` (break `/Game/DynamicCookingSystem/Blueprints/CookingInventory/F_ItemDetailsStruct` _itemdetails)) "NewEnumerator1")
          (`/Game/DynamicCookingSystem/Blueprints/CookingInventory/AC_CookingInventory.AddToInventory` _inventorycomponent (make `/Game/DynamicCookingSystem/Blueprints/CookingInventory/F_InventorySlotStruct` _itemdetails 1))
          (`self.K2_DestroyActor` _array_element_2)))
      (`KismetArrayLibrary.Array_Clear` (`self.ChunksInTheMixer`)))))

(event `self.MixerBoxCollision.OnComponentBeginOverlap`
  (params (OverlappedComponent :type "PrimitiveComponent Object Reference") (OtherActor :type "Actor Object Reference") (OtherComp :type "PrimitiveComponent Object Reference") (OtherBodyIndex :type Integer) (bFromSweep :type Boolean) (SweepResult :type "HitResult Structure (by ref)"))
  (bind _chunksinthemixer (`self.ChunksInTheMixer`))
  (bind _asbp_chunk (cast `/Game/DynamicCookingSystem/Blueprints/ParentActors/BP_Chunk` OtherActor))
  (`KismetArrayLibrary.Array_Add` _chunksinthemixer _asbp_chunk)
  (if (== (`KismetArrayLibrary.Array_LastIndex` _chunksinthemixer) 2)
    (`self.SetChunksMaterials`))
  (if (`self.IsRunning`)
    (if (`self.LidOpen`)
      (`/Game/DynamicCookingSystem/Blueprints/ParentActors/BP_Chunk.MixFX` _asbp_chunk)
      (`self.K2_DestroyActor` _asbp_chunk)
      (`KismetArrayLibrary.Array_RemoveItem` (`self.ChunksInTheMixer`) _asbp_chunk))))

(event `self.OnButton.OnBeginCursorOver`
  (params (TouchedComponent :type "PrimitiveComponent Object Reference"))
  (switch `/Game/DynamicCookingSystem/Data/E_CookingMode` (`/Game/DynamicCookingSystem/Blueprints/BP_CookingStation.CookingMode` (`self.CookingStationRef`))
    (:`NewEnumerator2`
      (bind _returnvalue (`|CreateWidget` "/Game/DynamicCookingSystem/Widgets/WBP_CookingUINameWidget.WBP_CookingUINameWidget_C" null "Off" "On"))
      (bind _output_get (set `self.UINameWidget` _returnvalue))
      (`UserWidget.AddToViewport` _output_get 0)
      (`/Game/DynamicCookingSystem/Widgets/WBP_CookingUINameWidget.SetWidget` _output_get (`self.IsRunning`)))))

(event `self.OnButton.OnEndCursorOver`
  (params (TouchedComponent :type "PrimitiveComponent Object Reference"))
  (switch `/Game/DynamicCookingSystem/Data/E_CookingMode` (`/Game/DynamicCookingSystem/Blueprints/BP_CookingStation.CookingMode` (`self.CookingStationRef`))
    (:`NewEnumerator2`
      (`Widget.RemoveFromParent` (`self.UINameWidget`)))))

(event `self.OpenLidButton.OnBeginCursorOver`
  (params (TouchedComponent :type "PrimitiveComponent Object Reference"))
  (switch `/Game/DynamicCookingSystem/Data/E_CookingMode` (`/Game/DynamicCookingSystem/Blueprints/BP_CookingStation.CookingMode` (`self.CookingStationRef`))
    (:`NewEnumerator2`
      (bind _returnvalue (`|CreateWidget` "/Game/DynamicCookingSystem/Widgets/WBP_CookingUINameWidget.WBP_CookingUINameWidget_C" null "Close" "Open"))
      (bind _output_get (set `self.UINameWidget` _returnvalue))
      (`UserWidget.AddToViewport` _output_get 0)
      (`/Game/DynamicCookingSystem/Widgets/WBP_CookingUINameWidget.SetWidget` _output_get (`self.LidOpen`)))))

(event `self.OpenLidButton.OnEndCursorOver`
  (params (TouchedComponent :type "PrimitiveComponent Object Reference"))
  (switch `/Game/DynamicCookingSystem/Data/E_CookingMode` (`/Game/DynamicCookingSystem/Blueprints/BP_CookingStation.CookingMode` (`self.CookingStationRef`))
    (:`NewEnumerator2`
      (`Widget.RemoveFromParent` (`self.UINameWidget`)))))

(event `/Game/DynamicCookingSystem/Blueprints/Interface/BI_Interact.Interact`
  (`/Game/DynamicCookingSystem/Blueprints/BP_CookingStation.StartCooking` (`self.CookingStationRef`)))

(fn `SetChunksMaterials`
  (bind _chunksinthemixer (`self.ChunksInTheMixer`))
  (bind _output (`|GetArrayItem` _chunksinthemixer))
  (`/Engine/EditorBlueprintResources/StandardMacros.IsValid` _output
    (:`Is Valid`
      (bind _returnvalue (`MaterialInstanceDynamic.K2_GetVectorParameterValue` (`/Game/DynamicCookingSystem/Blueprints/ParentActors/BP_Chunk.MaterialInstance` _output) "Color"))
      (set `self.Color3` _returnvalue)
      (bind _returnvalue_2 (`MaterialInstanceDynamic.K2_GetVectorParameterValue` (`/Game/DynamicCookingSystem/Blueprints/ParentActors/BP_Chunk.MaterialInstance` (`|GetArrayItem` _chunksinthemixer 1)) "Color"))
      (set `self.Color2` _returnvalue_2)
      (bind _returnvalue_3 (`MaterialInstanceDynamic.K2_GetVectorParameterValue` (`/Game/DynamicCookingSystem/Blueprints/ParentActors/BP_Chunk.MaterialInstance` (`|GetArrayItem` _chunksinthemixer 2)) "Color"))
      (set `self.Color1` _returnvalue_3))))

(fn `UserConstructionScript`)