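; Interactable cooking station where the player cuts, mixes and grills inventory ingredients.
; Interacting hands input to the station, opens the cooking widget and blends between cameras for each mode.
; SpawnIngredient places items at the cutting spawner or the child mixer and grill actors.
; Cutting slices procedural meshes along a switchable plane via mouse traces, up to a chunk limit; chunks or returned items go back to inventory.
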(event Custom|StartCooking
  (bind _returnvalue (Game|GetPlayerController 0))
  (bind _returnvalue_2 (Game|GetPlayerController 0))
  (Variables|Default|SetInUse? true)
  (Variables|/Script/Engine.PlayerController|SetbShowMouseCursor _returnvalue_2 true)
  (Variables|/Script/Engine.PlayerController|SetbEnableClickEvents _returnvalue_2 true)
  (Variables|/Script/Engine.PlayerController|SetbEnableMouseOverEvents _returnvalue_2 true)
  (Input|SetInputModeGameandUI _returnvalue_2 0 "DoNotLock" false false)
  (Game|Player|SetViewTargetwithBlend (Game|GetPlayerController 0) (Components|GetOwner (Variables|Default|GetMainCamera)) 1.0 "VTBlend_Linear" 0.0 false)
  (Input|DisableInput (Game|GetPlayerCharacter 0) _returnvalue)
  (Input|EnableInput _returnvalue)
  (Class|GameplayStatics|SetViewportMouseCaptureMode "CapturePermanently_IncludingInitialMouseDown")
  (CallFunction|CreateWidget)
  (bind _crosshair_widget (Class|BIGetData|GetCrosshair(Message) (Game|GetPlayerCharacter 0)))
  (Widget|SetVisibility _crosshair_widget "Collapsed"))

(event Custom|CreateWidget
  (bind _returnvalue (Game|GetPlayerController 0))
  (bind _returnvalue_2 (UserInterface|CreateWidget "/Game/DynamicCookingSystem/Widgets/WBP_CookingWidget.WBP_CookingWidget_C" 0 self))
  (bind _output_get (Variables|Default|SetCookingWidget _returnvalue_2))
  (UserInterface|Viewport|AddtoViewport _output_get 0)
  (Variables|/Script/Engine.PlayerController|SetbShowMouseCursor _returnvalue true)
  (Input|SetInputModeGameandUI _returnvalue 0 "DoNotLock" false false))

(event Custom|CookingAction
  (switch Utilities|FlowControl|Switch|SwitchonE_CookingMode (Variables|Default|GetCookingMode)
    (:NewEnumerator1
      (CallFunction|SwitchCamera (Variables|/Script/Engine.ChildActorComponent|GetChildActor (Variables|Default|GetCuttingCam))))
    (:NewEnumerator2
      (CallFunction|SwitchCamera (Variables|/Script/Engine.ChildActorComponent|GetChildActor (Variables|Default|GetMixingCam))))
    (:NewEnumerator3
      (CallFunction|SwitchCamera (Variables|/Script/Engine.ChildActorComponent|GetChildActor (Variables|Default|GetGrillingCam))))))

(event Custom|TakeAll
  (bind _sliced_actor (Variables|Default|GetSliced%20Actor))
  (bind _inventorycomponent (Class|BIGetData|GetInventory(Message) (Game|GetPlayerCharacter 0)))
  (Default|InsertIntoInventory _inventorycomponent (Utilities|Text|FormatText "{a} chunk" (.name (Variables|/Game/DynamicCookingSystem/Blueprints/ParentActors/BP_SliceableActor.BP_SliceableActor_C|GetItemDetails _sliced_actor))) "/Game/DynamicCookingSystem/Blueprints/ParentActors/BP_Chunk.BP_Chunk_C" true "/Game/DynamicCookingSystem/Textures/T_Square.T_Square" (Variables|/Game/DynamicCookingSystem/Blueprints/ParentActors/BP_SliceableActor.BP_SliceableActor_C|GetChunksAmount _sliced_actor) "NewEnumerator1" (Variables|/Game/DynamicCookingSystem/Blueprints/ParentActors/BP_SliceableActor.BP_SliceableActor_C|GetInsideMaterial _sliced_actor))
  (Actor|DestroyActor _sliced_actor))

(event Custom|HideProgressWidget
  (bind _as_wbp_progressbar (Variables|Default|GetAs%20WBP%20ProgressBar))
  (Widget|SetVisibility _as_wbp_progressbar "Collapsed")
  (Default|UpdateValue _as_wbp_progressbar 0.0))

(event Custom|SwitchCamera
  (params (Camera :type Actor%20Object%20Reference))
  (Game|Player|SetViewTargetwithBlend (Game|GetPlayerController 0) Camera 1.0 "VTBlend_Linear" 0.0 false))

(event Custom|QuitCooking
  (bind _returnvalue (Game|GetPlayerController 0))
  (bind _returnvalue_2 (Game|GetPlayerCharacter 0))
  (bind _returnvalue_3 (Game|GetPlayerController 0))
  (Input|EnableInput (Game|GetPlayerCharacter 0) _returnvalue_3)
  (Input|DisableInput _returnvalue_3)
  (Input|SetInputModeGameOnly _returnvalue false)
  (Variables|Default|SetInUse? false)
  (Variables|/Script/Engine.PlayerController|SetbShowMouseCursor _returnvalue false)
  (Pawn|Components|CharacterMovement|SetMovementMode (Variables|/Script/Engine.Character|GetCharacterMovement _returnvalue_2) "MOVE_Walking" 0)
  (Game|Player|SetViewTargetwithBlend (Game|GetPlayerController 0) _returnvalue_2 1.0 "VTBlend_Cubic" 0.0 true)
  (Widget|RemovefromParent (Variables|Default|GetCookingWidget))
  (Variables|Default|SetCookingMode "NewEnumerator0")
  (bind _crosshair_widget (Class|BIGetData|GetCrosshair(Message) (Game|GetPlayerCharacter 0)))
  (Widget|SetVisibility _crosshair_widget "Visible"))

(event Input|EnhancedActionEvents|EnhancedInputActionIA_Quit
  (params (ActionValue :type Boolean) (ElapsedSeconds :type Float%20%28double-precision%29) (TriggeredSeconds :type Float%20%28double-precision%29) (InputAction :type Input%20Action%20Object%20Reference :default "/Game/DynamicCookingSystem/Demo/5/ThirdPerson/Input/Actions/IA_Quit.IA_Quit"))
  (bind _returnvalue (Game|GetPlayerController 0))
  (bind _returnvalue_2 (Game|GetPlayerCharacter 0))
  (bind _returnvalue_3 (Game|GetPlayerController 0))
  (:Started
    (Input|EnableInput (Game|GetPlayerCharacter 0) _returnvalue_3)
    (Input|DisableInput _returnvalue_3)
    (Input|SetInputModeGameOnly _returnvalue false)
    (Variables|Default|SetInUse? false)
    (Variables|/Script/Engine.PlayerController|SetbShowMouseCursor _returnvalue false)
    (Pawn|Components|CharacterMovement|SetMovementMode (Variables|/Script/Engine.Character|GetCharacterMovement _returnvalue_2) "MOVE_Walking" 0)
    (Game|Player|SetViewTargetwithBlend (Game|GetPlayerController 0) _returnvalue_2 1.0 "VTBlend_Cubic" 0.0 true)
    (Widget|RemovefromParent (Variables|Default|GetCookingWidget))
    (Variables|Default|SetCookingMode "NewEnumerator0")
    (bind _crosshair_widget (Class|BIGetData|GetCrosshair(Message) (Game|GetPlayerCharacter 0)))
    (Widget|SetVisibility _crosshair_widget "Visible")))

(event EventBeginPlay
  (Utilities|FlowControl|Sequence
    (:then_0
      (bind _asbp_mixer (Utilities|Casting|CastToBP_Mixer (Variables|/Script/Engine.ChildActorComponent|GetChildActor (Variables|Default|GetMixer))))
      (Variables|/Game/DynamicCookingSystem/Blueprints/Mixer/BP_Mixer.BP_Mixer_C|SetCookingStationRef _asbp_mixer self)
      (Variables|Default|SetBP%20Mixer _asbp_mixer))
    (:then_1
      (bind _asbp_grill (Utilities|Casting|CastToBP_Grill (Variables|/Script/Engine.ChildActorComponent|GetChildActor (Variables|Default|GetGrill))))
      (Variables|/Game/DynamicCookingSystem/Blueprints/Grill/BP_Grill.BP_Grill_C|SetCookingStationRef _asbp_grill self)
      (Variables|Default|SetBP%20Grill _asbp_grill))
    (:then_2
      (bind _aswbp_progress_bar (Utilities|Casting|CastToWBP_ProgressBar (UserInterface|GetUserWidgetObject (Variables|Default|GetWidget))))
      (bind _output_get (Variables|Default|SetAs%20WBP%20ProgressBar _aswbp_progress_bar))
      (Variables|/Game/DynamicCookingSystem/Widgets/Timer/WBP_ProgressBar.WBP_ProgressBar_C|SetCookingStationRef _aswbp_progress_bar self)
      (Widget|SetVisibility _output_get "Collapsed"))))

(event EventInteract
  (CallFunction|StartCooking))

(event Custom|ResetCick
  (Utilities|FlowControl|DoOnce false) ; enters at Reset
)

(event Input|EnhancedActionEvents|EnhancedInputActionIA_Rotate
  (params (ActionValue :type Boolean) (ElapsedSeconds :type Float%20%28double-precision%29) (TriggeredSeconds :type Float%20%28double-precision%29) (InputAction :type Input%20Action%20Object%20Reference :default "/Game/DynamicCookingSystem/Demo/5/ThirdPerson/Input/Actions/IA_Rotate.IA_Rotate"))
  (:Started
    (Utilities|FlowControl|FlipFlop
      (:A
        (Variables|Default|SetCutRotation "0.000000,-180.000000,0.000000"))
      (:B
        (Variables|Default|SetCutRotation "-180.000000,0.000000,0.300000")))))

(event Input|EnhancedActionEvents|EnhancedInputActionIA_LeftClick
  (params (ActionValue :type Boolean) (ElapsedSeconds :type Float%20%28double-precision%29) (TriggeredSeconds :type Float%20%28double-precision%29) (InputAction :type Input%20Action%20Object%20Reference :default "/Game/DynamicCookingSystem/Demo/5/ThirdPerson/Input/Actions/IA_LeftClick.IA_LeftClick"))
  (bind _returnvalue (Game|GetPlayerController 0))
  (bind _returnvalue_2 (Math|Float|MakeLiteralFloat 1e+04))
  (bind (_worldlocation _worlddirection) (Game|Player|ConvertMouseLocationToWorldSpace _returnvalue))
  (bind _returnvalue_3 (* _worlddirection _returnvalue_2))
  (bind _returnvalue_4 (+ _returnvalue_3 _worldlocation))
  (:Started
    (switch Utilities|FlowControl|Switch|SwitchonE_CookingMode (Variables|Default|GetCookingMode)
      (:NewEnumerator1
        (if (not (Variables|Default|GetCuttingInProgress))
          (bind (_outhit _returnvalue_5) (Collision|LineTraceByChannel _worldlocation (Math|Vector|MakeVector (.x _returnvalue_4) (.y _returnvalue_4) (+ (.z _returnvalue_4) 6e+01)) "TraceTypeQuery1" false 0 "None"))
          (if _returnvalue_5
            (bind _asbp_sliceable_actor (Utilities|Casting|CastToBP_SliceableActor (.HitActor (Collision|BreakHitResult _outhit))))
            (if (not (>= (Variables|/Game/DynamicCookingSystem/Blueprints/ParentActors/BP_SliceableActor.BP_SliceableActor_C|GetChunksAmount _asbp_sliceable_actor) (Variables|Default|GetChunksMax)))
              (Variables|Default|SetSliced%20Actor _asbp_sliceable_actor)
              (Utilities|IsValid _asbp_sliceable_actor
                (:Is%20Valid
                  (Default|SliceWhole _asbp_sliceable_actor (.ImpactPoint (Collision|BreakHitResult _outhit)) (Variables|Default|GetCutRotation) (Variables|/Game/DynamicCookingSystem/Blueprints/ParentActors/BP_SliceableActor.BP_SliceableActor_C|GetProceduralMesh _asbp_sliceable_actor) (.HitComponent (Collision|BreakHitResult _outhit)))
                  (Default|AddChunk _asbp_sliceable_actor (Variables|Default|GetAs%20WBP%20ProgressBar))
                  (Variables|Default|SetCuttingInProgress true)
                  (Utilities|FlowControl|Delay 0.5)
                  (Variables|Default|SetCuttingInProgress false))))))))))

(event Input|EnhancedActionEvents|EnhancedInputActionIA_RIghtClick
  (params (ActionValue :type Boolean) (ElapsedSeconds :type Float%20%28double-precision%29) (TriggeredSeconds :type Float%20%28double-precision%29) (InputAction :type Input%20Action%20Object%20Reference :default "/Game/DynamicCookingSystem/Demo/5/ThirdPerson/Input/Actions/IA_RIghtClick.IA_RIghtClick"))
  (:Started
    (switch Utilities|FlowControl|Switch|SwitchonE_CookingMode (Variables|Default|GetCookingMode))))

(fn ConstructionScript)

(fn SpawnObjecttoSlice
  (params (Class :type BP%20Sliceable%20Actor%20Class%20Reference))
  (bind _sliced_actor (Variables|Default|GetSliced%20Actor))
  (Utilities|IsValid _sliced_actor
    (:Is%20Valid
      (if (Utilities|Array|IsEmpty (Variables|/Game/DynamicCookingSystem/Blueprints/ParentActors/BP_SliceableActor.BP_SliceableActor_C|GetChunks _sliced_actor))
        _
        (else
          (return false))))
    (:Is%20Not%20Valid
      _))
  (Utilities|IsValid (Variables|Default|GetSlicableActorRef)
    (:Is%20Valid
      (LocalVariables|SetNewLocalVar false)
      (Actor|DestroyActor (Variables|Default|GetSlicableActorRef)))
    (:Is%20Not%20Valid
      (LocalVariables|SetNewLocalVar true)))
  (Default|ResetProgressBar (Variables|Default|GetAs%20WBP%20ProgressBar))
  (bind _returnvalue (Game|SpawnActorfromClass Class (Math|Transform|MakeTransform (Transformation|GetWorldLocation (Variables|Default|GetSlicingActorSpawner)) "0, 0, 0" "1.000000,1.000000,1.000000") "Undefined" "SelectDefaultAtRuntime" 0 0))
  (Variables|Default|SetSlicableActorRef _returnvalue)
  (Widget|SetVisibility (Variables|Default|GetAs%20WBP%20ProgressBar) "HitTestInvisible")
  (return (LocalVariables|GetNewLocalVar)))

(fn SpawnObjecttoMix
  (params (Class :type BP%20Chunk%20Class%20Reference))
  (Game|SpawnActorfromClass Class (Math|Transform|MakeTransform (Transformation|GetWorldLocation (Variables|/Game/DynamicCookingSystem/Blueprints/Mixer/BP_Mixer.BP_Mixer_C|GetMixingActorSpawner (Variables|Default|GetBP%20Mixer))) "0, 0, 0" "1.000000,1.000000,1.000000") "Undefined" "SelectDefaultAtRuntime" 0 0)
  (return))

(fn SpawnObjecttoGrill
  (params (Class :type BP%20Mixed%20Actor%20Class%20Reference))
  (bind _bp_grill (Variables|Default|GetBP%20Grill))
  (Game|SpawnActorfromClass Class (Math|Transform|MakeTransform (Transformation|GetWorldLocation (select (Variables|/Game/DynamicCookingSystem/Blueprints/Grill/BP_Grill.BP_Grill_C|GetFirstSpanwerInUse _bp_grill) (Variables|/Game/DynamicCookingSystem/Blueprints/Grill/BP_Grill.BP_Grill_C|GetGrillActorSpawner _bp_grill) (Variables|/Game/DynamicCookingSystem/Blueprints/Grill/BP_Grill.BP_Grill_C|GetGrillActorSpawner2 _bp_grill))) "0, 0, 0" "1.000000,1.000000,1.000000") "Undefined" "SelectDefaultAtRuntime" 0 0)
  (return))

(fn SpawnIngredient
  (params (ActorClass :type Actor%20Class%20Reference) (ItemDetailsStruct :type F%20Item%20Details%20Struct%20Structure) (Index :type Integer) (CookingButton :type WBP%20Cooking%20Button%20Object%20Reference))
  (bind (_name _class _isstackable _icon _foodtype _chunkmaterial _color1 _color2 _color3) (Utilities|Struct|BreakF_ItemDetailsStruct ItemDetailsStruct))
  (bind _bp_grill (Variables|Default|GetBP%20Grill))
  (bind _amount (Variables|/Game/DynamicCookingSystem/Widgets/WBP_CookingButton.WBP_CookingButton_C|GetAmount CookingButton))
  (switch Utilities|FlowControl|Switch|SwitchonE_CookingMode (Variables|Default|GetCookingMode)
    (:NewEnumerator1
      (Default|ResetProgressBar (Variables|Default|GetAs%20WBP%20ProgressBar))
      (bind _returnvalue (Game|SpawnActorfromClass ActorClass (Math|Transform|MakeTransform (Transformation|GetWorldLocation (Variables|Default|GetSlicingActorSpawner)) "0, 0, 0" "1.000000,1.000000,1.000000") "Undefined" "SelectDefaultAtRuntime" 0 0))
      (bind _output_get (Variables|Default|SetSpawnedActor _returnvalue))
      (Class|BISetMaterial|SetIndex(Message) _output_get Index)
      (Variables|Default|SetLastIndex Index)
      (Variables|Default|SetLastItemDetails ItemDetailsStruct)
      (Widget|SetVisibility (Variables|Default|GetAs%20WBP%20ProgressBar) "HitTestInvisible")
      (Variables|Default|SetLastAmount Index)
      (return _output_get))
    (:NewEnumerator2
      (bind _returnvalue_2 (Game|SpawnActorfromClass ActorClass (Math|Transform|MakeTransform (Transformation|GetWorldLocation (Variables|/Game/DynamicCookingSystem/Blueprints/Mixer/BP_Mixer.BP_Mixer_C|GetMixingActorSpawner (Variables|Default|GetBP%20Mixer))) "0, 0, 0" "1.000000,1.000000,1.000000") "Undefined" "SelectDefaultAtRuntime" 0 0))
      (Class|BISetMaterial|SetMaterials(Message) _returnvalue_2 _chunkmaterial)
      (Class|BISetMaterial|SetIndex(Message) _returnvalue_2 Index)
      (Class|BISetMaterial|SetDetails(Message) _returnvalue_2 ItemDetailsStruct)
      (Variables|Default|SetLastAmount _amount)
      (return _returnvalue_2))
    (:NewEnumerator3
      (bind _returnvalue_3 (Game|SpawnActorfromClass ActorClass (Math|Transform|MakeTransform (Transformation|GetWorldLocation (select (Variables|/Game/DynamicCookingSystem/Blueprints/Grill/BP_Grill.BP_Grill_C|GetFirstSpanwerInUse _bp_grill) (Variables|/Game/DynamicCookingSystem/Blueprints/Grill/BP_Grill.BP_Grill_C|GetGrillActorSpawner _bp_grill) (Variables|/Game/DynamicCookingSystem/Blueprints/Grill/BP_Grill.BP_Grill_C|GetGrillActorSpawner2 _bp_grill))) "0, 0, 0" "1.000000,1.000000,1.000000") "Undefined" "SelectDefaultAtRuntime" 0 0))
      (Class|BISetMaterial|SetColors(Message) _returnvalue_3 _color1 _color2 _color3)
      (Variables|Default|SetLastAmount _amount)
      (return _returnvalue_3))))

(fn ReturnItem
  (bind _lastindex (Variables|Default|GetLastIndex))
  (bind _inventorycomponent (Class|BIGetData|GetInventory(Message) (Game|GetPlayerCharacter 0)))
  (if (== (Variables|Default|GetLastAmount) 0)
    (Default|AddtoInventory _inventorycomponent (Utilities|Struct|MakeF_InventorySlotStruct (.itemdetails (Utilities|Struct|MakeF_InventorySlotStruct (Variables|Default|GetLastItemDetails))) 1))
    (Actor|DestroyActor (Variables|Default|GetSpawnedActor))
    (elif (Utilities|Array|IsValidIndex (Variables|/Game/DynamicCookingSystem/Blueprints/CookingInventory/AC_CookingInventory.AC_CookingInventory_C|GetInventory _inventorycomponent) _lastindex)
      (Default|AddtoInventory _inventorycomponent (Utilities|Struct|MakeF_InventorySlotStruct (.itemdetails (Utilities|Array|Get(acopy) (Variables|/Game/DynamicCookingSystem/Blueprints/CookingInventory/AC_CookingInventory.AC_CookingInventory_C|GetInventory _inventorycomponent) _lastindex)) 1))
      (Actor|DestroyActor (Variables|Default|GetSpawnedActor))
      (else
        (Default|AddtoInventory _inventorycomponent (Utilities|Struct|MakeF_InventorySlotStruct (.itemdetails (Utilities|Struct|MakeF_InventorySlotStruct (Variables|Default|GetLastItemDetails))) 1))
        (Actor|DestroyActor (Variables|Default|GetSpawnedActor))))))