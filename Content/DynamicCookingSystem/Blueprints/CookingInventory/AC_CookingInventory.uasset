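; Inventory component for the cooking system that stores ingredient slots, each holding item details and a quantity.
; Adding merges stackable items into a slot with matching name and class, otherwise inserts a new slot at the front.
; Removing decrements a slot's quantity and deletes it at zero.
; It also fills a wrap box with cooking buttons for items of a given food type, linked to a cooking station.
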(event `self.ReceiveBeginPlay`)

(fn `AddToInventory`
  (params (ItemToAdd :type "/Game/DynamicCookingSystem/Blueprints/CookingInventory/F_InventorySlotStruct Structure"))
  (if (`.IsStackable_11_84986D654B6FE61C6B1F0AB009AC8E9D` (break `/Game/DynamicCookingSystem/Blueprints/CookingInventory/F_ItemDetailsStruct` (`.ItemDetails_8_E8C9C29049842C5491FF62AC1A4E20C6` (break `/Game/DynamicCookingSystem/Blueprints/CookingInventory/F_InventorySlotStruct` ItemToAdd))))
    (bind _stackindex (`self.HasPartialStack` ItemToAdd)
      (:`True`
        (`self.AddToStack` ItemToAdd _stackindex))
      (:`False`
        (`self.CreateStack2` ItemToAdd :!label _label)))
    (else
      (goto _label))))

(fn `AddToInventory2`
  (params (ItemToAdd :type "/Game/DynamicCookingSystem/Blueprints/CookingInventory/F_InventorySlotStruct Structure"))
  (if (`.IsStackable_11_84986D654B6FE61C6B1F0AB009AC8E9D` (break `/Game/DynamicCookingSystem/Blueprints/CookingInventory/F_ItemDetailsStruct` (`.ItemDetails_8_E8C9C29049842C5491FF62AC1A4E20C6` (break `/Game/DynamicCookingSystem/Blueprints/CookingInventory/F_InventorySlotStruct` ItemToAdd))))
    (bind _stackindex (`self.HasPartialStack` ItemToAdd)
      (:`True`
        (`self.AddToStack` ItemToAdd _stackindex))
      (:`False`
        (`self.CreateStack2` (struct) :!label _label)))
    (else
      (goto _label))))

(fn `AddToStack`
  (params (SlotStructure :type "/Game/DynamicCookingSystem/Blueprints/CookingInventory/F_InventorySlotStruct Structure") (SlotIndex :type Integer))
  (locals (CurrentStackQuiantity :type Integer))
  (bind (_itemdetails _quantity) (break `/Game/DynamicCookingSystem/Blueprints/CookingInventory/F_InventorySlotStruct` SlotStructure))
  (bind (_output_itemdetails _output_quantity) (break `/Game/DynamicCookingSystem/Blueprints/CookingInventory/F_InventorySlotStruct` (`|GetArrayItem` (`self.Inventory`) SlotIndex)))
  (bind _output_get (set `local.CurrentStackQuiantity` _output_quantity))
  (`KismetArrayLibrary.Array_Set` (`self.Inventory`) SlotIndex (make `/Game/DynamicCookingSystem/Blueprints/CookingInventory/F_InventorySlotStruct` _itemdetails (+ _output_get _quantity))))

(fn `CreateStack`
  (params (ItemToAdd :type "/Game/DynamicCookingSystem/Blueprints/CookingInventory/F_InventorySlotStruct Structure"))
  (`KismetArrayLibrary.Array_Add` (`self.Inventory`) ItemToAdd))

(fn `CreateStack2`
  (params (ItemToAdd :type "/Game/DynamicCookingSystem/Blueprints/CookingInventory/F_InventorySlotStruct Structure"))
  (`KismetArrayLibrary.Array_Insert` (`self.Inventory`) ItemToAdd))

(fn `InsertIntoInventory`
  (params (Name :type Text) (Class :type "Actor Class Reference") (IsStackable :type Boolean) (Icon :type "Texture2D Object Reference") (Quantity :type Integer) (`Food Type` :type "/Game/DynamicCookingSystem/Blueprints/CookingInventory/E_FoodType Enum" :default "NewEnumerator0") (ChunkMaterial :type "MaterialInterface Object Reference") (Color1 :type "LinearColor Structure") (Color2 :type "LinearColor Structure") (Color3 :type "LinearColor Structure"))
  (`self.AddToInventory` (make `/Game/DynamicCookingSystem/Blueprints/CookingInventory/F_InventorySlotStruct` (make `/Game/DynamicCookingSystem/Blueprints/CookingInventory/F_ItemDetailsStruct` Name Class IsStackable Icon `Food Type` ChunkMaterial Color1 Color2 Color3) Quantity)))

(fn `PopulateShelfWithButtons`
  (params (WrapBoxRef :type "WrapBox Object Reference") (CookinStation :type "/Game/DynamicCookingSystem/Blueprints/BP_CookingStation Object Reference") (FoodType :type "/Game/DynamicCookingSystem/Blueprints/CookingInventory/E_FoodType Enum" :default "NewEnumerator0"))
  (`PanelWidget.ClearChildren` WrapBoxRef)
  (for (_array_element _array_index) (`self.Inventory`)
    (bind (_itemdetails _quantity) (break `/Game/DynamicCookingSystem/Blueprints/CookingInventory/F_InventorySlotStruct` _array_element))
    (bind (_name _class _isstackable _icon _foodtype) (break `/Game/DynamicCookingSystem/Blueprints/CookingInventory/F_ItemDetailsStruct` _itemdetails))
    (if (`|EnumEquality` _foodtype FoodType)
      (bind _returnvalue (`|CreateWidget` "/Game/DynamicCookingSystem/Widgets/WBP_CookingButton.WBP_CookingButton_C"))
      (`WrapBox.SetInnerSlotPadding` WrapBoxRef (5.0 5.0))
      (`WrapBox.AddChildToWrapBox` WrapBoxRef _returnvalue)
      (set `/Game/DynamicCookingSystem/Widgets/WBP_CookingButton.CookinStation` CookinStation _returnvalue)
      (set `/Game/DynamicCookingSystem/Widgets/WBP_CookingButton.Name` _name _returnvalue)
      (set `/Game/DynamicCookingSystem/Widgets/WBP_CookingButton.Amount` _quantity _returnvalue)
      (set `/Game/DynamicCookingSystem/Widgets/WBP_CookingButton.Ingredient to Spawn` _class _returnvalue)
      (set `/Game/DynamicCookingSystem/Widgets/WBP_CookingButton.Texture` _icon _returnvalue)
      (`/Game/DynamicCookingSystem/Widgets/WBP_CookingButton.SetButton` _returnvalue)
      (set `/Game/DynamicCookingSystem/Widgets/WBP_CookingButton.Index` _array_index _returnvalue)
      (set `/Game/DynamicCookingSystem/Widgets/WBP_CookingButton.ItemDetails` _itemdetails _returnvalue))))

(fn `RemoveFromInventory`
  (params (Index :type Integer))
  (bind (_output_itemdetails _output_quantity) (break `/Game/DynamicCookingSystem/Blueprints/CookingInventory/F_InventorySlotStruct` (`|GetArrayItem` (`self.Inventory`) Index)))
  (`KismetArrayLibrary.Array_Set` (`self.Inventory`) Index (make `/Game/DynamicCookingSystem/Blueprints/CookingInventory/F_InventorySlotStruct` _output_itemdetails (- _output_quantity 1)))
  (if (== _output_quantity 0)
    (`KismetArrayLibrary.Array_Remove` (`self.Inventory`) Index)))