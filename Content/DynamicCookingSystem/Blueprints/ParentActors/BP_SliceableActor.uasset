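; Parent actor for sliceable items in the cooking system, which can also be picked up into the player's inventory.
; Construction copies the configured static mesh into a procedural mesh for runtime cutting.
; Debounced slice events cut the mesh or a hit chunk, adding capped physics halves with impulse, sound and FX.
; Chunk counting feeds a progress bar and destroys the actor at zero, while cursor hover shows a name widget.
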(event `SliceAction`
  (params (PlanePosition :type "Vector Structure") (PlaneNormal :type "Vector Structure") (InProcMesh :type "ProceduralMeshComponent Object Reference"))
  (`self.CutFX` PlanePosition)
  (bind _outotherhalfprocmesh (`KismetProceduralMeshLibrary.SliceProceduralMesh` InProcMesh PlanePosition PlaneNormal true "CreateNewSectionForCap" (`self.InsideMaterial`)))
  (`PrimitiveComponent.SetSimulatePhysics` _outotherhalfprocmesh true)
  (`PrimitiveComponent.SetCollisionEnabled` _outotherhalfprocmesh "QueryAndPhysics")
  (`PrimitiveComponent.AddImpulse` _outotherhalfprocmesh (10.0 0.0 150.0) "None" true)
  (`KismetArrayLibrary.Array_Add` (`self.Chunks`) _outotherhalfprocmesh))

(event `SliceWhole`
  (params (PlanePosition :type "Vector Structure") (PlaneNormal :type "Vector Structure") (InProcMesh :type "ProceduralMeshComponent Object Reference") (HitComponent :type "PrimitiveComponent Object Reference"))
  (if (`KismetArrayLibrary.Array_IsEmpty` (`self.Chunks`))
    (`/Engine/EditorBlueprintResources/StandardMacros.DoOnce` false :!label _label
      (:`Completed`
        (`self.SliceAction` PlanePosition PlaneNormal InProcMesh)
        (`KismetSystemLibrary.Delay` 0.5)
        (goto _label :!via `Reset`)))
    (else
      (for _array_element (`self.Chunks`)
        (if (== HitComponent _array_element)
          (`/Engine/EditorBlueprintResources/StandardMacros.DoOnce` false :!label _label_2
            (:`Completed`
              (`self.SliceAction` PlanePosition PlaneNormal _array_element)
              (`KismetSystemLibrary.Delay` 0.5)
              (goto _label_2 :!via `Reset`)))
          (else
            (goto _label)))))))

(event `AddChunk`
  (params (ProgressBar :type "/Game/DynamicCookingSystem/Widgets/Timer/WBP_ProgressBar Object Reference"))
  (`/Engine/EditorBlueprintResources/StandardMacros.IncrementInt` (`self.ChunksAmount`)
    (:`  `
      (`/Game/DynamicCookingSystem/Widgets/Timer/WBP_ProgressBar.AddProgress` ProgressBar))))

(event `ChunksCheck`
  (params (Widget :type "/Game/DynamicCookingSystem/Widgets/WBP_CookingWidget Object Reference"))
  (bind _result (`/Engine/EditorBlueprintResources/StandardMacros.DecrementInt` (`self.ChunksAmount`))
    (:`  `
      (if (<= _result 0)
        (`KismetSystemLibrary.Delay` 0.5)
        (`self.K2_DestroyActor`)))))

(event `CutFX`
  (params (Location :type "Vector Structure") (Rotation :type "Rotator Structure"))
  (`GameplayStatics.PlaySound2D` (`self.CutSound`) 1.0 1.0 0.0 null null)
  (`NiagaraFunctionLibrary.SpawnSystemAtLocation` (`self.FXEffect`) Location Rotation))

(event `Chunked`
  (`PrimitiveComponent.SetCollisionEnabled` (`self.ProceduralMesh`) "QueryOnly"))

(event `self.ProceduralMesh.OnBeginCursorOver`
  (params (TouchedComponent :type "PrimitiveComponent Object Reference"))
  (bind _returnvalue (`|CreateWidget` "/Game/DynamicCookingSystem/Widgets/WBP_CookingUINameWidget.WBP_CookingUINameWidget_C" null "Cut" "Cut"))
  (bind _output_get (set `self.UINameWidget` _returnvalue))
  (`UserWidget.AddToViewport` _output_get 0)
  (`/Game/DynamicCookingSystem/Widgets/WBP_CookingUINameWidget.SetWidget` _output_get false))

(event `self.ProceduralMesh.OnEndCursorOver`
  (params (TouchedComponent :type "PrimitiveComponent Object Reference"))
  (`Widget.RemoveFromParent` (`self.UINameWidget`)))

(event `/Game/DynamicCookingSystem/Blueprints/Interface/BI_Interact.Interact`
  (bind _inventorycomponent (message `/Game/DynamicCookingSystem/Blueprints/Interface/BI_GetData.GetInventory` (`GameplayStatics.GetPlayerCharacter` 0)))
  (`/Game/DynamicCookingSystem/Blueprints/CookingInventory/AC_CookingInventory.AddToInventory` _inventorycomponent (make `/Game/DynamicCookingSystem/Blueprints/CookingInventory/F_InventorySlotStruct` (`self.ItemDetails`) 1))
  (`self.K2_DestroyActor`))

(event `/Game/DynamicCookingSystem/Blueprints/Interface/BI_Interact.RemoveFromInventory`
  (params (Dex :type Integer))
  (bind _inventorycomponent (message `/Game/DynamicCookingSystem/Blueprints/Interface/BI_GetData.GetInventory` (`GameplayStatics.GetPlayerCharacter` 0)))
  (`/Game/DynamicCookingSystem/Blueprints/CookingInventory/AC_CookingInventory.RemoveFromInventory` _inventorycomponent Dex))

(event `/Game/DynamicCookingSystem/Blueprints/Interface/BI_SetMaterial.SetIndex`
  (params (Index :type Integer))
  (set `self.Index` Index))

(fn `GetIndex`
  (returns (Index :type Integer))
  (return (`self.Index`)))

(fn `Slicing`
  (params (InProcMesh :type "ProceduralMeshComponent Object Reference") (PlanePosition :type "Vector Structure") (PlaneNormal :type "Vector Structure") (Force :type "Vector Structure") (CapMaterial :type "MaterialInterface Object Reference"))
  (bind _outotherhalfprocmesh (`KismetProceduralMeshLibrary.SliceProceduralMesh` InProcMesh PlanePosition PlaneNormal true "CreateNewSectionForCap" CapMaterial))
  (`PrimitiveComponent.SetSimulatePhysics` _outotherhalfprocmesh true)
  (`PrimitiveComponent.SetCollisionEnabled` _outotherhalfprocmesh "QueryAndPhysics")
  (`PrimitiveComponent.AddForce` _outotherhalfprocmesh Force "None" true)
  (`KismetArrayLibrary.Array_Add` (`self.Chunks`) _outotherhalfprocmesh))

(fn `UserConstructionScript`
  (bind _staticmesh (`self.StaticMesh`))
  (`StaticMeshComponent.SetStaticMesh` _staticmesh (`self.ActorStaticMesh`))
  (`PrimitiveComponent.SetMaterial` _staticmesh 0 (`self.ActorMaterial`))
  (`KismetProceduralMeshLibrary.CopyProceduralMeshFromStaticMeshComponent` (`self.StaticMesh`) 0 (`self.ProceduralMesh`) true)
  (`ActorComponent.K2_DestroyComponent` (`self.StaticMesh`)))