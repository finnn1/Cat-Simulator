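; Parent actor for a mixed food mass in the cooking system, clickable to take or flip depending on the station's mode.
; In Mixing it enters the inventory as "Mixed Mass" with its three material colors.
; In Grilling a widget timer gates an animated flip and, once flipped, pickup as "Cooked".
; Timelines drive per-side material alphas for browning, alongside grilling sound, smoke and a hover label.
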(event `self.ReceiveBeginPlay`
  (bind _aswbp_timer (cast `/Game/DynamicCookingSystem/Widgets/Timer/WBP_Timer` (`WidgetComponent.GetUserWidgetObject` (`self.TimerWidget`))))
  (bind _output_get (set `self.WBP Timer` _aswbp_timer))
  (set `/Game/DynamicCookingSystem/Widgets/Timer/WBP_Timer.CookingStationRef` (`self.CookingStation`) _output_get)
  (`Widget.SetVisibility` _output_get "Hidden"))

(event `StartGrilling`
  (bind _wbp_timer (`self.WBP Timer`))
  (bind _staticmesh (`self.StaticMesh`))
  (`AudioComponent.FadeIn` (`self.GrillingSound`) 0.1 1.0 0.0 "Linear")
  (`/Game/DynamicCookingSystem/Widgets/Timer/WBP_Timer.ResetTimer` _wbp_timer)
  (`Widget.SetVisibility` _wbp_timer "Visible")
  (`/Game/DynamicCookingSystem/Widgets/Timer/WBP_Timer.StartTimer` _wbp_timer 5.0)
  (if (`self.Fliped`)
    (bind (_direction _time) (`Timeline|Timeline`)
      (:`Update`
        (`MeshComponent.SetScalarParameterValueOnMaterials` _staticmesh "Alpha" _time)
        (`MeshComponent.SetScalarParameterValueOnMaterials` _staticmesh "DropsAlpha" _time)))
    (else
      (bind (_direction_2 _time_2) (`Timeline|GrillTimeline`)
        (:`Update`
          (`MeshComponent.SetScalarParameterValueOnMaterials` (`self.StaticMesh`) "Alpha2" _time_2))
        (:`Finished`
          (`ActorComponent.Activate` (`self.Smoke`) false))))))

(event `self.StaticMesh.OnClicked`
  (params (TouchedComponent :type "PrimitiveComponent Object Reference") (ButtonPressed :type "Key Structure"))
  (bind _uinamewidget (`self.UINameWidget`))
  (bind _uinamewidget_2 (`self.UINameWidget`))
  (switch `/Game/DynamicCookingSystem/Data/E_CookingMode` (`/Game/DynamicCookingSystem/Blueprints/BP_CookingStation.CookingMode` (`self.CookingStation`))
    (:`NewEnumerator2`
      (`/Engine/EditorBlueprintResources/StandardMacros.IsValid` _uinamewidget_2
        (:`Is Valid`
          (`Widget.RemoveFromParent` _uinamewidget_2))
        (:`Is Not Valid`
          _))
      (`self.AddMixedToInventory`)
      (`self.K2_DestroyActor`))
    (:`NewEnumerator3`
      (if (`/Game/DynamicCookingSystem/Widgets/Timer/WBP_Timer.Ready` (`self.WBP Timer`))
        (if (`self.Fliped`)
          (`/Engine/EditorBlueprintResources/StandardMacros.IsValid` _uinamewidget
            (:`Is Valid`
              (`Widget.RemoveFromParent` _uinamewidget))
            (:`Is Not Valid`
              _))
          (`self.AddMixedToInventoryCooked`)
          (`self.K2_DestroyActor`)
          (else
            (`self.Flip`)))))))

(event `MaterialRotation`)

(event `self.StaticMesh.OnBeginCursorOver`
  (params (TouchedComponent :type "PrimitiveComponent Object Reference"))
  (switch `/Game/DynamicCookingSystem/Data/E_CookingMode` (`/Game/DynamicCookingSystem/Blueprints/BP_CookingStation.CookingMode` (`self.CookingStation`))
    (:`NewEnumerator2`
      (bind _returnvalue (`|CreateWidget` "/Game/DynamicCookingSystem/Widgets/WBP_CookingUINameWidget.WBP_CookingUINameWidget_C" null "Flip" "Take"))
      (bind _output_get (set `self.UINameWidget` _returnvalue))
      (`UserWidget.AddToViewport` _output_get 0)
      (`/Game/DynamicCookingSystem/Widgets/WBP_CookingUINameWidget.SetWidget` _output_get (`self.OnGrill`)))
    (:`NewEnumerator3`
      (bind _returnvalue_2 (`|CreateWidget` "/Game/DynamicCookingSystem/Widgets/WBP_CookingUINameWidget.WBP_CookingUINameWidget_C" null "Take" "Flip"))
      (bind _output_get_2 (set `self.UINameWidget` _returnvalue_2))
      (`UserWidget.AddToViewport` _output_get_2 0)
      (`/Game/DynamicCookingSystem/Widgets/WBP_CookingUINameWidget.SetWidget` _output_get_2 (and (`/Game/DynamicCookingSystem/Widgets/Timer/WBP_Timer.Ready` (`self.WBP Timer`)) (`self.Fliped`))))))

(event `self.StaticMesh.OnEndCursorOver`
  (params (TouchedComponent :type "PrimitiveComponent Object Reference"))
  (switch `/Game/DynamicCookingSystem/Data/E_CookingMode` (`/Game/DynamicCookingSystem/Blueprints/BP_CookingStation.CookingMode` (`self.CookingStation`))
    (:`NewEnumerator2`
      _)
    (:`NewEnumerator3`
      _))
  (`Widget.RemoveFromParent` (`self.UINameWidget`)))

(event `/Game/DynamicCookingSystem/Blueprints/Interface/BI_Interact.RemoveFromInventory`
  (params (Dex :type Integer))
  (bind _inventorycomponent (message `/Game/DynamicCookingSystem/Blueprints/Interface/BI_GetData.GetInventory` (`GameplayStatics.GetPlayerCharacter` 0)))
  (`/Game/DynamicCookingSystem/Blueprints/CookingInventory/AC_CookingInventory.RemoveFromInventory` _inventorycomponent Dex))

(event `/Game/DynamicCookingSystem/Blueprints/Interface/BI_SetMaterial.SetColors`
  (params (Color1 :type "LinearColor Structure") (Color2 :type "LinearColor Structure") (Color3 :type "LinearColor Structure"))
  (`self.SetMaterial` Color1 Color2 Color3))

(event `Flip`
  (bind _staticmesh (`self.StaticMesh`))
  (bind _staticmesh_2 (`self.StaticMesh`))
  (bind (_relativelocation_x _relativelocation_y _relativelocation_z) (`KismetMathLibrary.BreakVector` (`SceneComponent.RelativeLocation` _staticmesh)))
  (bind (_relativelocation_x_2 _relativelocation_y_2 _relativelocation_z_2) (`KismetMathLibrary.BreakVector` (`SceneComponent.RelativeLocation` _staticmesh_2)))
  (if (`self.CanFlip`)
    _
    (elif (`/Game/DynamicCookingSystem/Blueprints/Grill/BP_Grill.IsRunning` (`/Game/DynamicCookingSystem/Blueprints/BP_CookingStation.BP Grill` (`self.CookingStation`)))
      (`|ExecutionSequence`
        (:`then_0`
          (set `self.CanFlip` true)
          (`AudioComponent.FadeOut` (`self.GrillingSound`) 0.1 0.0 "Linear")
          (`PrimitiveComponent.SetSimulatePhysics` _staticmesh_2 false)
          (`KismetSystemLibrary.MoveComponentTo` _staticmesh_2 (`KismetMathLibrary.MakeVector` _relativelocation_x_2 _relativelocation_y_2 (+ _relativelocation_z_2 25.0)) (struct :`Roll` 180.0) true true 0.5)
          (`KismetSystemLibrary.MoveComponentTo` _staticmesh (`KismetMathLibrary.MakeVector` _relativelocation_x _relativelocation_y (- _relativelocation_z 25.0)) (struct :`Roll` 180.0) true true 0.5)
          (`PrimitiveComponent.SetSimulatePhysics` _staticmesh_2 true)
          (`AudioComponent.FadeIn` (`self.GrillingSound`) 0.1 1.0 0.0 "Linear")
          (set `self.Fliped` (not (`self.Fliped`)))
          (if (`/Game/DynamicCookingSystem/Blueprints/Grill/BP_Grill.IsRunning` (`/Game/DynamicCookingSystem/Blueprints/BP_CookingStation.BP Grill` (`self.CookingStation`)))
            (`self.StartGrilling`)
            (set `self.CanFlip` false)))
        (:`then_1`
          (`self.MaterialRotation`))))))

(fn `AddMixedToInventory`
  (bind _inventorycomponent (message `/Game/DynamicCookingSystem/Blueprints/Interface/BI_GetData.GetInventory` (`GameplayStatics.GetPlayerCharacter` 0)))
  (`/Game/DynamicCookingSystem/Blueprints/CookingInventory/AC_CookingInventory.InsertIntoInventory` _inventorycomponent "Mixed Mass" "BP_MixedActor_C" false "/Game/DynamicCookingSystem/Textures/T_Mixed.T_Mixed" 1 "NewEnumerator2" null (`self.Color1`) (`self.Color2`) (`self.Color3`))
  (`/Game/DynamicCookingSystem/Widgets/WBP_Shelf.PopulateShelf` (`/Game/DynamicCookingSystem/Widgets/WBP_CookingWidget.WBP_Shelf` (`/Game/DynamicCookingSystem/Blueprints/BP_CookingStation.CookingWidget` (`self.CookingStation`))) "NewEnumerator2")
  (`/Game/DynamicCookingSystem/Widgets/WBP_Shelf.PopulateShelf` (`/Game/DynamicCookingSystem/Widgets/WBP_CookingWidget.WBP_Shelf` (`/Game/DynamicCookingSystem/Blueprints/BP_CookingStation.CookingWidget` (`self.CookingStation`))) "NewEnumerator1"))

(fn `AddMixedToInventoryCooked`
  (bind _inventorycomponent (message `/Game/DynamicCookingSystem/Blueprints/Interface/BI_GetData.GetInventory` (`GameplayStatics.GetPlayerCharacter` 0)))
  (`/Game/DynamicCookingSystem/Blueprints/CookingInventory/AC_CookingInventory.InsertIntoInventory` :`self` _inventorycomponent :`Name` "Cooked" :`Class` "BP_MixedActor_C" :`IsStackable` true :`Quantity` 1 :`Food Type` "NewEnumerator3"))

(fn `GetIndex`
  (returns (Index :type Integer))
  (return 0))

(fn `SetMaterial`
  (params (InLinearColor :type "LinearColor Structure") (InLinearColor1 :type "LinearColor Structure") (InLinearColor2 :type "LinearColor Structure"))
  (bind _staticmesh (`self.StaticMesh`))
  (set `self.Color1` InLinearColor)
  (set `self.Color2` InLinearColor1)
  (set `self.Color3` InLinearColor2)
  (`MeshComponent.SetVectorParameterValueOnMaterials` _staticmesh "Color1" (`KismetMathLibrary.Conv_LinearColorToVector` InLinearColor))
  (`MeshComponent.SetVectorParameterValueOnMaterials` _staticmesh "Color2" (`KismetMathLibrary.Conv_LinearColorToVector` InLinearColor1))
  (`MeshComponent.SetVectorParameterValueOnMaterials` _staticmesh "Color3" (`KismetMathLibrary.Conv_LinearColorToVector` InLinearColor2)))

(fn `UserConstructionScript`)