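; BP_Chunk is an actor in the dynamic cooking system that represents a chunk with a static mesh, an index and item details.
; The construction script applies its default material, and SetMaterials swaps it and stores a dynamic material instance.
; MixFX plays a 2D sound and spawns an effect at the chunk.
; RemovefromInventory forwards an index to the player character's inventory, while simple setters and GetIndex expose the stored data.
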(event `MixFX`
  (`GameplayStatics.PlaySound2D` (`self.MixSound`) 1.0 1.0 0.0 null null)
  (`NiagaraFunctionLibrary.SpawnSystemAtLocation` (`self.FXEffect`) (`self.K2_GetActorLocation`) (`self.K2_GetActorRotation`)))

(event `/Game/DynamicCookingSystem/Blueprints/Interface/BI_SetMaterial.SetMaterials`
  (params (Material :type "MaterialInterface Object Reference"))
  (`PrimitiveComponent.SetMaterial` (`self.StaticMesh`) 0 Material)
  (bind _returnvalue (`PrimitiveComponent.CreateDynamicMaterialInstance` (`self.StaticMesh`) 0 Material "None"))
  (set `self.MaterialInstance` _returnvalue))

(event `/Game/DynamicCookingSystem/Blueprints/Interface/BI_Interact.RemoveFromInventory`
  (params (Dex :type Integer))
  (bind _inventorycomponent (message `/Game/DynamicCookingSystem/Blueprints/Interface/BI_GetData.GetInventory` (`GameplayStatics.GetPlayerCharacter` 0)))
  (`/Game/DynamicCookingSystem/Blueprints/CookingInventory/AC_CookingInventory.RemoveFromInventory` _inventorycomponent Dex))

(event `/Game/DynamicCookingSystem/Blueprints/Interface/BI_SetMaterial.SetIndex`
  (params (Index :type Integer))
  (set `self.Index` Index))

(event `/Game/DynamicCookingSystem/Blueprints/Interface/BI_SetMaterial.SetDetails`
  (params (ItemDetailsStruct :type "/Game/DynamicCookingSystem/Blueprints/CookingInventory/F_ItemDetailsStruct Structure"))
  (set `self.Item Details Struct` ItemDetailsStruct))

(fn `GetIndex`
  (returns (Index :type Integer))
  (return (`self.Index`)))

(fn `UserConstructionScript`
  (`PrimitiveComponent.SetMaterial` (`self.StaticMesh`) 0 (`self.Actor Material`)))