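; Actor component that turns its owner into a fishable area, keeping it stocked with fish that can seek bait.
; On BeginPlay and each bait alert, it refills empty FishPool slots with fish using random data, spawned at random points within the owner's bounds.
; AlertFish waits a random time from the bait ID's range, or a default range, then sends the nearest fish to the bait.
; Rarity and size weighting is only noted, not implemented.
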(event `self.ReceiveBeginPlay`
  ;[0.05098 0.05098 0.05098] Reset Fish Pool
  (`self.Reset Fish Pool`))

(event `AlertFish`
  (params (Bait :type "/Game/FPSFishing/Blueprints/Fishing/BP_FishingBait_asset Object Reference"))
  (bind _bait (`self.Bait`))
  (bind _returnvalue (`Actor.K2_GetActorLocation` _bait))
  (bind (_value _returnvalue_2) (`BlueprintMapLibrary.Map_Find` (`self.FishingTime`) (`/Game/FPSFishing/Blueprints/Fishing/BP_FishingBait_asset.BaitId` (`self.Bait`))))
  (bind _fish (`self.FindNearestFish` _returnvalue))
  (bind (_x _y) (`KismetMathLibrary.BreakVector2D` _value))
  ;[0.05098 0.05098 0.05098] Alert Fish
  (bind _output_get (set `self.Bait` Bait))
  (`/Engine/EditorBlueprintResources/StandardMacros.IsValid` _output_get
    (:`Is Valid`
      (`self.Reset Fish Pool`)
      (if _returnvalue_2
        (`KismetSystemLibrary.Delay` (`KismetMathLibrary.RandomFloatInRange` _x _y))
        (else
          (`KismetSystemLibrary.Delay` (`KismetMathLibrary.RandomFloatInRange` (`self.DefaultMinTimeToFindBait`) (`self.DefaultMaxTimeToFindBait`)))))
      (`/Engine/EditorBlueprintResources/StandardMacros.IsValid` _bait
        (:`Is Valid`
          (`/Engine/EditorBlueprintResources/StandardMacros.IsValid` _fish
            (:`Is Valid`
              (`/Game/FPSFishing/Blueprints/Fishing/BP_Fish_asset.FindBait` _fish _returnvalue))))))))

(fn `FindNearestFish`
  (params (Origin :type "Vector Structure"))
  (returns (Fish :type "/Game/FPSFishing/Blueprints/Fishing/BP_Fish_asset Object Reference"))
  (bind _asbp_fish_asset (cast `/Game/FPSFishing/Blueprints/Fishing/BP_Fish_asset` (`.ReturnValue` (`GameplayStatics.FindNearestActor` Origin (`self.FishPool`)))))
  (return _asbp_fish_asset))

(fn `GetRandomPointInBounds`
  (returns (ReturnValue :type "Vector Structure"))
  (bind (_origin _boxextent) (`Actor.GetActorBounds` (`self.GetOwner`) false false))
  (return (`KismetMathLibrary.RandomPointInBoundingBox` _origin _boxextent)))

(fn `Reset Fish Pool`
  (`KismetArrayLibrary.Array_Resize` (`self.FishPool`) (`self.FishAmount`))
  (for (_array_element _array_index) (`self.FishPool`)
    (`/Engine/EditorBlueprintResources/StandardMacros.IsValid` _array_element
      (:`Is Not Valid`
        (bind _returnvalue (`self.Spawn Fish`))
        (`KismetArrayLibrary.Array_Set` (`self.FishPool`) _array_index _returnvalue)))))

(fn `Spawn Fish`
  (returns (ReturnValue :type "/Game/FPSFishing/Blueprints/Fishing/BP_Fish_asset Object Reference"))
  (bind _returnvalue (`|SpawnActorFromClass` "/Game/FPSFishing/Blueprints/Fishing/BP_Fish_asset.BP_Fish_asset_C" (`KismetMathLibrary.MakeTransform` (`self.GetRandomPointInBounds`)) "Undefined" "OverrideRootScale" (`self.GetOwner`) (`KismetArrayLibrary.Array_Random` (`self.FishData`)) null))
  (return _returnvalue))