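; Fishing component for the player pawn that manages bait, casting and the start and end of a fishing session.
; Casting traces the rod's predicted throw, requires a hit on a fishable-area component, spawns hidden bait if none is attached, and locks player movement.
; Outcomes go out through dispatchers, and an eaten bait lets the fish escape after a delay.
; The catch QTE widget logic is disconnected and the aim-spline function is empty.
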(event `OnFishCaughtEvent`
  (params (Fish :type "/Game/FPSFishing/Blueprints/Fishing/BP_Fish_asset Object Reference"))
  ;[0.05098 0.05098 0.05098] OnBaitEaten
  (`/Engine/EditorBlueprintResources/StandardMacros.IsValid` Fish
    (:`Is Valid`
      (`/Game/FPSFishing/Blueprints/Fishing/BP_Fish_asset.OnCaught` Fish)
      (`self.OnFishCaught` Fish))))

(event `self.ReceiveBeginPlay`
  ;[0.05098 0.05098 0.05098] OnBaitEaten
  ;;[0.05098 0.05098 0.05098] BeginPlay
  (`self.CacheOwnerController`))

(event `OnFishEscapedEvent`
  (params (Fish :type "/Game/FPSFishing/Blueprints/Fishing/BP_Fish_asset Object Reference"))
  ;[0.05098 0.05098 0.05098] OnBaitEaten
  (`/Engine/EditorBlueprintResources/StandardMacros.IsValid` Fish
    (:`Is Valid`
      (`/Game/FPSFishing/Blueprints/Fishing/BP_Fish_asset.OnEscaped` Fish)
      (`self.OnFishEscaped` Fish))))

(event `OnBaitEaten`
  (params (Bait :type "/Game/FPSFishing/Blueprints/Fishing/BP_FishingBait_asset Object Reference") (Fish :type "/Game/FPSFishing/Blueprints/Fishing/BP_Fish_asset Object Reference"))
  ;[0.05098 0.05098 0.05098] OnBaitEaten
  (`/Engine/EditorBlueprintResources/StandardMacros.IsValid` Bait
    (:`Is Valid`
      (`/Engine/EditorBlueprintResources/StandardMacros.IsValid` Fish
        (:`Is Valid`
          (set `self.bEaten` true)
          (`KismetSystemLibrary.Delay` 5.0)
          (if (`self.bEaten`)
            (`/Game/FPSFishing/Blueprints/Fishing/BP_Fish_asset.OnEscaped` Fish)
            (set `self.bEaten` false)))))))

(fn `AddAimSplinePointsFromTracedPath`
  (params (PathPositions :type "Array of Vector Structure") (bSuccessfulTrace :type Boolean)))

(fn `Aim`
  (returns (TargetLocation :type "Vector Structure") (ReturnValue :type Boolean))
  (if (not (`self.bFishing`))
    (bind (_outhit _outpathpositions _impactpoint _returnvalue) (`self.PathTraceFishingTrajectory`))
    (`self.AddAimSplinePointsFromTracedPath` _outpathpositions _returnvalue)
    (return _impactpoint _returnvalue)))

(fn `AttachBait`
  (params (Bait :type "/Game/FPSFishing/Blueprints/Fishing/BP_FishingBait_asset Object Reference"))
  (`/Engine/EditorBlueprintResources/StandardMacros.IsValid` Bait
    (:`Is Valid`
      (bind _rod (`self.Rod`)
        (:`then`
          (bind _balreadyattached (`/Game/LSU/Blueprints/Fishing/BP_FishingRod.AttachBait` _rod (`local.Bait`)))
          (if (not _balreadyattached)
            (add `/Game/FPSFishing/Blueprints/Fishing/BP_FishingBait_asset.OnBaitEaten` (`local.Bait`) (`|CreateDelegate` :!event `OnBaitEaten`))
            (`self.OnBaitAttached` (`local.Bait`))))
        (:`else`)))))

(fn `AttachBaitQuickly`
  (params (Bait :type "/Game/FPSFishing/Blueprints/Fishing/BP_FishingBait_asset Object Reference"))
  (`/Engine/EditorBlueprintResources/StandardMacros.IsValid` Bait
    (:`Is Valid`
      (bind _rod (`self.Rod`)
        (:`then`
          (bind _balreadyattached (`/Game/LSU/Blueprints/Fishing/BP_FishingRod.AttachBait` _rod (`local.Bait`)))
          (if (not _balreadyattached)
            (add `/Game/FPSFishing/Blueprints/Fishing/BP_FishingBait_asset.OnBaitEaten` (`local.Bait`) (`|CreateDelegate` :!event `OnBaitEaten`))
            (`Actor.K2_AttachToComponent` (`local.Bait`) (`/Game/LSU/Blueprints/Fishing/BP_FishingRod.Mesh` (`self.Rod`)) "FishHangingSocket" "SnapToTarget" "SnapToTarget" "KeepRelative" true)))
        (:`else`)))))

(fn `CacheOwnerController`
  (bind _ass_vrpawn_test (cast `/Game/VRTemplate/Blueprints/S_VRPawnTest` (`self.GetOwner`)))
  (set `self.OwnerController` (`Pawn.GetController` _ass_vrpawn_test)))

(fn `CanCast`
  (returns (ReturnValue :type Boolean))
  (return (and (not (`self.bFishing`)) (`KismetSystemLibrary.IsValid` (`self.Rod`)) (not (`self.IsOwnerPlayingMontage`)) (not (`.bFound` (`self.FindFishBeingCaught`))) (`KismetMathLibrary.Vector_IsZero` (`Actor.GetVelocity` (`self.GetOwner`))))))

(fn `Cast`
  (returns (bSuccess :type Boolean))
  (if (`self.CanCast`)
    (bind (_targetlocation _returnvalue) (`self.Aim`))
    (if _returnvalue
      (`self.StartFishing`)
      (return true)
      (else
        _)))
  (`self.OnCastFailed`)
  (return false))

(fn `ChangeBait`
  (params (Id :type Name))
  (set `self.BaitToUse` Id)
  (set `self.bRefreshBait` true)
  (`self.ChangeBaitSpawn`))

(fn `ChangeBaitSpawn`
  (if (`self.bRefreshBait`)
    (if (== (`self.BaitToUse`) "NoBait")
      _
      (elif (`self.IsActive`)
        (bind _rod (`self.Rod`)
          (:`then`
            (`/Engine/EditorBlueprintResources/StandardMacros.IsValid` (`/Game/LSU/Blueprints/Fishing/BP_FishingRod.GetBait` _rod)
              (:`Is Not Valid`
                (bind _returnvalue (`|SpawnActorFromClass` "/Game/FPSFishing/Blueprints/Fishing/BP_FishingBait_asset.BP_FishingBait_asset_C" (`KismetMathLibrary.MakeTransform` (0.0 0.0 0.0) (struct) (0.05 0.05 0.05)) "Undefined" "OverrideRootScale" (`self.Rod`) (`self.BaitToUse`) (`Actor.Instigator` (`self.GetOwner`)))) ; Get Inventory Bait
                (`self.AttachBait` _returnvalue)
                (set `self.bRefreshBait` false))))
          (:`else`))))))

(fn `EndFishing`
  (bind _returnvalue (`Actor.GetComponentByClass` (`self.GetOwner`) "/Script/Engine.CharacterMovementComponent"))
  (set `self.bFishing` false)
  (bind _ownercontroller (`self.OwnerController`)
    (:`then`
      (bind _asplayer_controller (cast `PlayerController` _ownercontroller))
      (`WidgetBlueprintLibrary.SetInputMode_GameOnly` _asplayer_controller)
      (`Controller.ResetIgnoreMoveInput` _asplayer_controller)
      (`/Engine/EditorBlueprintResources/StandardMacros.IsValid` _returnvalue
        (:`Is Valid`
          (`CharacterMovementComponent.SetMovementMode` _returnvalue "MOVE_Walking" 0)
          (`|ExecutionSequence`
            (:`then_0`
              (bind _asbp_character_fishing (cast `/Game/FPSFishing/Blueprints/BP_CharacterFishing` (`GameplayStatics.GetPlayerCharacter` 0)))
              (set `/Game/FPSFishing/Blueprints/BP_CharacterFishing.bFishingCamera` false _asbp_character_fishing))
            (:`then_1`
              (set `self.BaitToUse` "None"))))))
    (:`else`)))

(fn `EndFishingQuickly`
  (if (and (`self.bFishing`) (not (`self.IsOwnerPlayingMontage`)) (`KismetSystemLibrary.IsValid` (`self.Rod`)) (`KismetMathLibrary.Vector_IsZero` (`Actor.GetVelocity` (`self.GetOwner`))))
    (`self.OnFishEscaped` null)
    (bind _rod (`self.Rod`)
      (:`then`
        (bind _fishing_bait (`/Game/LSU/Blueprints/Fishing/BP_FishingRod.GetBait` _rod))
        (`/Engine/EditorBlueprintResources/StandardMacros.IsValid` _fishing_bait
          (:`Is Valid`
            (`Actor.K2_DestroyActor` _fishing_bait))))
      (:`else`))))

(fn `FindFishBeingCaught`
  (returns (Fish :type "/Game/FPSFishing/Blueprints/Fishing/BP_Fish_asset Object Reference") (bFound :type Boolean))
  (bind _rod (`self.Rod`)
    (:`then`
      (bind _asbp_fish_asset (cast `/Game/FPSFishing/Blueprints/Fishing/BP_Fish_asset` (`CableComponent.GetAttachedActor` (`/Game/LSU/Blueprints/Fishing/BP_FishingRod.Cable` _rod)))
        (:`then`
          (return _asbp_fish_asset true))
        (:`CastFailed`
          _)))
    (:`else`
      _))
  (return null false))

(fn `IsOwnerPlayingMontage`
  (returns (ReturnValue :type Boolean))
  (bind _ascharacter (cast `Character` (`self.GetOwner`))
    (:`then`
      (return (`KismetSystemLibrary.IsValid` (`Character.GetCurrentMontage` _ascharacter))))
    (:`CastFailed`
      (return false))))

(fn `PathTraceFishingTrajectory`
  (returns (OutHit :type "HitResult Structure") (OutPathPositions :type "Array of Vector Structure") (ImpactPoint :type "Vector Structure") (ReturnValue :type Boolean))
  (locals (`Projectile Radius` :type "Float (single-precision)" :default 1.0))
  (bind _rod (`self.Rod`))
  (bind _rod_2 (`self.Rod`)
    (:`then`
      (bind (_startpos _launchvelocity) (`/Game/LSU/Blueprints/Fishing/BP_FishingRod.CalcThrowTrajectory` _rod_2))
      (bind (_outhit _outpathpositions) (`GameplayStatics.Blueprint_PredictProjectilePath_ByTraceChannel` _startpos _launchvelocity true (`local.Projectile Radius`) "ECC_Visibility" false (`|MakeArray` (`self.GetOwner`) _rod (`/Game/LSU/Blueprints/Fishing/BP_FishingRod.GetBait` _rod) :!type "Actor Object Reference") "None" 45.0 15.0 3.0))
      (bind (_bblockinghit _binitialoverlap _time _distance _location _impactpoint _normal _impactnormal _physmat _hitactor) (`GameplayStatics.BreakHitResult` _outhit))
      (`/Engine/EditorBlueprintResources/StandardMacros.IsValid` _hitactor
        (:`Is Valid`
          (return _outhit _outpathpositions _impactpoint (`KismetSystemLibrary.IsValid` (`Actor.GetComponentByClass` _hitactor "/Game/FPSFishing/Blueprints/Fishing/BP_FishableAreaComponent_asset.BP_FishableAreaComponent_asset_C"))))))
    (:`else`)))

(fn `ResetIgnoreLookInput`
  (`|ExecutionSequence`
    (:`then_0`
      (bind _asbp_character_fishing (cast `/Game/FPSFishing/Blueprints/BP_CharacterFishing` (`GameplayStatics.GetPlayerCharacter` 0)))
      (`/Game/FPSFishing/Blueprints/BP_CharacterFishing.SetFishingLook` _asbp_character_fishing))
    (:`then_1`
      (bind _ownercontroller (`self.OwnerController`)
        (:`then`
          (bind _asplayer_controller (cast `PlayerController` _ownercontroller))
          (`Controller.ResetIgnoreLookInput` _asplayer_controller))
        (:`else`)))))

(fn `SetRodSize`
  (params (Scale :type "Float (double-precision)"))
  (bind _rod (`self.Rod`)
    (:`then`
      (`/Game/LSU/Blueprints/Fishing/BP_FishingRod.SetSize` _rod Scale))
    (:`else`)))

(fn `StartFishing`
  (locals (Bait :type "/Game/FPSFishing/Blueprints/Fishing/BP_FishingBait_asset Object Reference"))
  (bind _returnvalue (`Actor.GetComponentByClass` (`self.GetOwner`) "/Script/Engine.CharacterMovementComponent"))
  (`GameplayStatics.PlaySound2D` "/Game/FPSFishing/Art/Audio/aim.aim" 1.0 1.0 0.0 null null)
  (bind _rod (`self.Rod`)
    (:`then`
      (bind _fishing_bait (`/Game/LSU/Blueprints/Fishing/BP_FishingRod.GetBait` _rod))
      (`/Engine/EditorBlueprintResources/StandardMacros.IsValid` _fishing_bait
        (:`Is Valid`
          (`self.OnCastSucceeded` _fishing_bait :!label _label)
          (set `self.bFishing` true)
          (bind _ownercontroller (`self.OwnerController`)
            (:`then`
              (bind _asplayer_controller (cast `PlayerController` _ownercontroller))
              (`Controller.SetIgnoreMoveInput` _asplayer_controller true)
              (`Controller.SetIgnoreLookInput` _asplayer_controller true)
              (`KismetSystemLibrary.K2_SetTimer` null "ResetIgnoreLookInput" 2.0)
              (`/Engine/EditorBlueprintResources/StandardMacros.IsValid` _returnvalue
                (:`Is Valid`
                  (`CharacterMovementComponent.DisableMovement` _returnvalue))))
            (:`else`)))
        (:`Is Not Valid`
          (bind _returnvalue_2 (`|SpawnActorFromClass` "/Game/FPSFishing/Blueprints/Fishing/BP_FishingBait_asset.BP_FishingBait_asset_C" (`KismetMathLibrary.MakeTransform` (0.0 0.0 0.0) (struct) (0.05 0.05 0.05)) "Undefined" "OverrideRootScale" (`self.Rod`) (`self.BaitToUse`) (`Actor.Instigator` (`self.GetOwner`))))
          (`Actor.SetActorHiddenInGame` _returnvalue_2 true)
          (`self.AttachBaitQuickly` _returnvalue_2)
          (`|ExecutionSequence`
            (:`then_0`
              (`/Game/LSU/Blueprints/Fishing/BP_FishingRod.ThrowBait` (`self.Rod`)))
            (:`then_1`
              (goto _label))))))
    (:`else`)))