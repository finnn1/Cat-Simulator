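; Fishing-game fish actor, built from its Data's mesh, size and speed, that swims as a dark silhouette until caught.
; Tick moves it between random points in its spawning owner's bounds, or toward bait once FindBait is called.
; On arrival a sphere trace either finds bait to eat, starting Escaping effects and notifying the bait, or resumes swimming.
; OnCaught reveals true colors and stops effects; OnEscaped detaches it back to swimming.
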(event `self.ReceiveBeginPlay`
  ;[0.05098 0.05098 0.05098] Init Target Location
  (set `self.TargetLocation` (`self.GetRandomPointInLake`)))

(event `self.ReceiveTick`
  (params (DeltaSeconds :type "Float (single-precision)"))
  ;[0.05098 0.05098 0.05098] Movement
  (if (`self.IsAtTargetLocation`)
    (switch `/Game/FPSFishing/Blueprints/Fishing/EFishState` (`self.State`)
      (:`NewEnumerator0`
        (set `self.TargetLocation` (`self.GetRandomPointInLake`)))
      (:`NewEnumerator1`
        (`self.OnBaitFindingFinished`)))
    (else
      (switch `/Game/FPSFishing/Blueprints/Fishing/EFishState` (`self.State`)
        (:`NewEnumerator0`
          _)
        (:`NewEnumerator1`
          _))
      (`self.Move Towards` (`self.TargetLocation`)))))

(fn `EatBait`
  (params (Bait :type "/Game/FPSFishing/Blueprints/Fishing/BP_FishingBait_asset Object Reference"))
  (`/Engine/EditorBlueprintResources/StandardMacros.IsValid` Bait
    (:`Is Valid`
      (`ActorComponent.Activate` (`self.RotatingMovement`) true)
      (`ActorComponent.Activate` (`self.Audio`) true)
      (set `self.State` "NewEnumerator2")
      (`/Game/FPSFishing/Blueprints/Fishing/BP_FishingBait_asset.OnEaten` (`local.Bait`) self)
      (`self.SpawnEscapingParticles`))))

(fn `FindBait`
  (params (Location :type "Vector Structure"))
  (set `self.TargetLocation` Location)
  (set `self.State` "NewEnumerator1")
  (`GameplayStatics.PlaySound2D` "/Game/FPSFishing/Art/Audio/FishAlert.FishAlert" 1.0 1.0 0.0 null null)
  (`self.SetActorTickEnabled` true)
  (`self.SetActorHiddenInGame` false))

(fn `GetCurrentStateSpeed`
  (returns (Speed :type "Float (double-precision)"))
  (locals (FindingBaitSpeedMultiplier :type "Float (double-precision)" :default 2.0) (PullSpeedMultiplier :type "Float (double-precision)" :default 4.0))
  (bind (_data_id _data_size _data_rarity _data_mesh _data_speed) (break `/Game/FPSFishing/Blueprints/Fishing/FFish` (`self.Data`)))
  (return (* _data_speed (select `/Game/FPSFishing/Blueprints/Fishing/EFishState` (`self.State`) :`NewEnumerator0` 1.0 :`NewEnumerator1` (`local.FindingBaitSpeedMultiplier`) :`NewEnumerator2` 1.0))))

(fn `GetRandomPointInLake`
  (returns (ReturnValue :type "Vector Structure"))
  (bind _returnvalue (`self.GetOwner`))
  (bind (_origin _boxextent) (`self.GetActorBounds` _returnvalue false false))
  (`/Engine/EditorBlueprintResources/StandardMacros.IsValid` _returnvalue
    (:`Is Valid`
      (return (`KismetMathLibrary.RandomPointInBoundingBox` _origin _boxextent)))))

(fn `InitFish`
  (bind (_data_id _data_size _data_rarity _data_mesh) (break `/Game/FPSFishing/Blueprints/Fishing/FFish` (`self.Data`)))
  (`StaticMeshComponent.SetStaticMesh` (`self.StaticMesh`) _data_mesh)
  (bind _returnvalue (`KismetMaterialLibrary.CreateDynamicMaterialInstance` (`StaticMesh.GetMaterial` _data_mesh 0)))
  (set `self.DynamicMaterial` _returnvalue)
  (`|ExecutionSequence`
    (:`then_0`
      (bind _dynamicmaterial (`self.DynamicMaterial`)
        (:`then`
          (`MaterialInstanceDynamic.SetVectorParameterValue` _dynamicmaterial "Tint" (struct :`A` 1.0))
          (`self.SetDynamicMaterialScalarParameter` "ColorMaskAlpha" 1.0) ; Add Color Mask
          (`PrimitiveComponent.SetMaterial` (`self.StaticMesh`) 0 _dynamicmaterial))
        (:`else`)))
    (:`then_1`
      (`self.SetActorScale3D` (`KismetMathLibrary.Conv_DoubleToVector` (`.Size_15_F8612C5F4C3C45ECED931D9CD9BE32D3` (break `/Game/FPSFishing/Blueprints/Fishing/FFish` (`self.Data`))))))))

(fn `IsAtTargetLocation`
  (returns (ReturnValue :type Boolean))
  (locals (Tolerance :type "Float (single-precision)" :default 10.0))
  (return (== (`self.K2_GetActorLocation`) (`self.TargetLocation`) :`ErrorTolerance` (`local.Tolerance`))))

(fn `Move Towards`
  (params (Target :type "Vector Structure"))
  (`self.K2_SetActorLocationAndRotation` (`KismetMathLibrary.VInterpTo_Constant` (`self.K2_GetActorLocation`) (`local.Target`) (`GameplayStatics.GetWorldDeltaSeconds`) (`self.GetCurrentStateSpeed`)) (`KismetMathLibrary.RInterpTo_Constant` (`self.K2_GetActorRotation`) (`KismetMathLibrary.FindLookAtRotation` (`self.K2_GetActorLocation`) (`local.Target`)) (`GameplayStatics.GetWorldDeltaSeconds`) (`self.GetCurrentStateSpeed`))))

(fn `OnBaitFindingFinished`
  (bind _returnvalue (`self.K2_GetActorLocation`))
  (bind _outhits (`KismetSystemLibrary.SphereTraceMulti` _returnvalue _returnvalue (`KismetMathLibrary.VSize` (`.BoxExtent` (`self.GetActorBounds` false))) "TraceTypeQuery1"))
  (for _array_element _outhits
    (bind _asbp_fishing_bait (cast `/Game/FPSFishing/Blueprints/Fishing/BP_FishingBait_asset` (`.HitActor` (`GameplayStatics.BreakHitResult` _array_element))))
    (`self.EatBait` _asbp_fishing_bait)
    (return))
  (`self.OnEscaped`)
  (return))

(fn `OnCaught`
  (bind _fishescparts (`self.FishEscParts`))
  (set `self.State` "NewEnumerator3")
  (`self.SetActorEnableCollision` false)
  (`|ExecutionSequence`
    (:`then_0`
      (bind _dynamicmaterial (`self.DynamicMaterial`)
        (:`then`
          (`MaterialInstanceDynamic.SetVectorParameterValue` _dynamicmaterial "Tint" (struct :`R` 1.0 :`G` 1.0 :`B` 1.0 :`A` 1.0)))
        (:`else`)))
    (:`then_1`
      (`self.SetDynamicMaterialScalarParameter` "WindIntensity") ; Stop Material Movement
      (`self.SetDynamicMaterialScalarParameter` "ColorMaskAlpha") ; Remove Color Mask
      (`PrimitiveComponent.SetRenderCustomDepth` (`self.StaticMesh`) false)
      (`ActorComponent.Deactivate` (`self.RotatingMovement`))
      (`ActorComponent.Deactivate` (`self.Audio`))
      (`KismetSystemLibrary.K2_ClearTimer` null "SpawnEscapingParticles")
      (`GameplayStatics.SpawnEmitterAttached` "/Game/FPSFishing/Art/VFX/PS_Splash1.PS_Splash1" (`self.StaticMesh`) "None" (0.0 0.0 0.0) (struct) (1.0 1.0 1.0) "SnapToTargetIncludingScale")
      (`/Engine/EditorBlueprintResources/StandardMacros.IsValid` _fishescparts
        (:`Is Valid`
          (`ActorComponent.Deactivate` _fishescparts))))))

(fn `OnEscaped`
  (bind _fishescparts (`self.FishEscParts`))
  (set `self.State` "NewEnumerator0")
  (`self.K2_DetachFromActor` "KeepWorld" "KeepWorld" "KeepWorld")
  (`ActorComponent.Deactivate` (`self.RotatingMovement`))
  (`ActorComponent.Deactivate` (`self.Audio`))
  (`/Engine/EditorBlueprintResources/StandardMacros.IsValid` _fishescparts
    (:`Is Valid`
      (`ActorComponent.Deactivate` _fishescparts))))

(fn `SetDynamicMaterialScalarParameter`
  (params (ParameterName :type Name) (Value :type "Float (single-precision)"))
  (bind _dynamicmaterial (`self.DynamicMaterial`)
    (:`then`
      (`MaterialInstanceDynamic.SetScalarParameterValue` _dynamicmaterial ParameterName Value))
    (:`else`)))

(fn `SpawnEscapingParticles`
  (bind _returnvalue (`GameplayStatics.SpawnEmitterAttached` "/Game/FPSFishing/Art/VFX/PS_ripples.PS_ripples" (`self.StaticMesh`) "None" (0.0 0.0 0.0) (struct) (1.0 1.0 1.0) "SnapToTargetIncludingScale"))
  (set `self.FishEscParts` _returnvalue))

(fn `UserConstructionScript`
  (`self.InitFish`))