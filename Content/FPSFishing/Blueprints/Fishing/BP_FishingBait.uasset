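; BP_FishingBait is the thrown bait actor that attracts and gets eaten by fish in the fishing game.
; Throw launches it with physics; on hit it alerts any fishable area component on the hit actor, then freezes with a plop and splash.
; When eaten, it fires a bait-eaten event, scales an emitter and instigator camera shake by fish size, then destroys itself.
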(event `self.StaticMesh.OnComponentHit`
  (params (HitComponent :type "PrimitiveComponent Object Reference") (OtherActor :type "Actor Object Reference") (OtherComp :type "PrimitiveComponent Object Reference") (NormalImpulse :type "Vector Structure") (Hit :type "HitResult Structure (by ref)"))
  (bind _returnvalue (`self.GetComponentByClass` OtherActor "/Game/FPSFishing/Blueprints/Fishing/BP_FishableAreaComponent.BP_FishableAreaComponent_C"))
  (bind _returnvalue_2 (`self.K2_GetActorLocation`))
  ;[0.05098 0.05098 0.05098] Stop physics simulation on hit
  (`self.PlayCamerashake` 0.5)
  (`/Engine/EditorBlueprintResources/StandardMacros.IsValid` _returnvalue
    (:`Is Valid`
      (`/Game/FPSFishing/Blueprints/Fishing/BP_FishableAreaComponent.AlertFish` _returnvalue self))
    (:`Is Not Valid`
      _))
  (if (`SceneComponent.IsSimulatingPhysics` (`self.StaticMesh`) "None")
    (`PrimitiveComponent.SetSimulatePhysics` (`self.StaticMesh`) false)
    (`GameplayStatics.PlaySoundAtLocation` "/Game/FPSFishing/Art/Audio/WaterPlop_Cue.WaterPlop_Cue" _returnvalue_2 (struct) 1.0 1.0 0.0 null null null null)
    (`GameplayStatics.SpawnEmitterAtLocation` "/Game/FPSFishing/Art/VFX/PS_Splash1.PS_Splash1" _returnvalue_2)))

(fn `OnEaten`
  (params (EatenBy :type "/Game/FPSFishing/Blueprints/Fishing/BP_Fish Object Reference"))
  (bind (_data_id _data_size) (break `/Game/FPSFishing/Blueprints/Fishing/FFish` (`/Game/FPSFishing/Blueprints/Fishing/BP_Fish.Data` EatenBy)))
  (`/Engine/EditorBlueprintResources/StandardMacros.IsValid` EatenBy
    (:`Is Valid`
      (`self.OnBaitEaten` self EatenBy)
      (`self.PlayCamerashake` _data_size)
      (`GameplayStatics.SpawnEmitterAtLocation` null (`self.K2_GetActorLocation`) (struct) (`KismetMathLibrary.Conv_DoubleToVector` _data_size))
      (`self.K2_DestroyActor`))))

(fn `PlayCamerashake`
  (params (Scale :type "Float (single-precision)" :default 1.0))
  (bind `_as플레이어_컨트롤러` (cast `PlayerController` (`self.GetInstigatorController`)))
  (`PlayerController.ClientStartCameraShake` :`self` `_as플레이어_컨트롤러` :`Shake` (`self.ShakeClass`) :`Scale` Scale))

(fn `Throw`
  (params (Velocity :type "Vector Structure"))
  (`PrimitiveComponent.SetSimulatePhysics` (`self.StaticMesh`) true)
  (`PrimitiveComponent.SetPhysicsLinearVelocity` (`self.StaticMesh`) Velocity false "None"))

(fn `UserConstructionScript`)