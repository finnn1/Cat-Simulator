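; Fishing rod Blueprint that holds and throws bait, reels in what the line catches, and previews the cast.
; A cable attaches to the bait, switches to whatever eats it, and a timeline pulls that actor to the rod before resetting.
; Throws use suggested projectile velocity along the view direction.
; While shown, the arc rebuilds spline meshes every tick from the predicted path, green over fishable areas, otherwise red.
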(event `Pull`
  (params (Rate :type "Float (single-precision)"))
  (bind _returnvalue (`CableComponent.GetAttachedActor` (`self.Cable`)))
  ;[0.05098 0.05098 0.05098] Pull
  (`TimelineComponent.SetPlayRate` (`self.PullTimeline`) Rate)
  (`/Engine/EditorBlueprintResources/StandardMacros.IsValid` _returnvalue
    (:`Is Valid`
      (set `self.Rot1` (`self.K2_GetActorRotation` _returnvalue))
      (bind (_direction _alpha) (`Timeline|PullTimeline` :!via `PlayFromStart` :!label _label)
        (:`Update`
          (`self.PullCable` _alpha))
        (:`Finished`
          (`self.ResetCable`))))
    (:`Is Not Valid`
      (goto _label :!via `PlayFromStart`))))

(event `self.ReceiveTick`
  (params (DeltaSeconds :type "Float (single-precision)"))
  (if (`self.bShowArc`)
    (`self.UpdateFishArc`)))

(event `self.ReceiveBeginPlay`
  (bind _returnvalue (`KismetMaterialLibrary.CreateDynamicMaterialInstance` "/Game/FPSFishing/Blueprints/Fishing/Arc/MI_SplineMat_Inst.MI_SplineMat_Inst"))
  (set `self.SplineMat` _returnvalue))

(fn `AttachBait`
  (params (Bait :type "/Game/FPSFishing/Blueprints/Fishing/BP_FishingBait_asset Object Reference"))
  (returns (bAlreadyAttached :type Boolean))
  (`/Engine/EditorBlueprintResources/StandardMacros.IsValid` (`self.GetBait`)
    (:`Is Valid`
      (return true))
    (:`Is Not Valid`
      (bind _output_get (set `self.Bait` Bait))
      (add `/Game/FPSFishing/Blueprints/Fishing/BP_FishingBait_asset.OnBaitEaten` _output_get (`|CreateDelegate` :!event `OnBaitEaten`))
      ;[0.05098 0.05098 0.05098] Attach bait to mesh
      (`self.K2_AttachToComponent` (`self.Bait`) (`self.Mesh`) "FishHangingSocket" "SnapToTarget" "SnapToTarget" "KeepWorld" true)
      ;[0.05098 0.05098 0.05098] Attach cable to bait
      (set `CableComponent.bAttachEnd` true (`self.Cable`))
      (`CableComponent.SetAttachEndToComponent` (`self.Cable`) (`/Game/FPSFishing/Blueprints/Fishing/BP_FishingBait_asset.StaticMesh` (`self.Bait`)) "None")
      ;[0.05098 0.05098 0.05098] Show Cable
      (`SceneComponent.SetVisibility` (`self.Cable`) true false)
      (return false))))

(fn `CalcThrowTrajectory`
  (returns (StartPos :type "Vector Structure") (LaunchVelocity :type "Vector Structure"))
  (locals (StartLocation :type "Vector Structure" :default (0.0 0.0 0.0)) (EndLocation :type "Vector Structure" :default (0.0 0.0 0.0)))
  (`self.Instigator`
    (:`then`
      ;[0.05098 0.05098 0.05098] Start Location from Rod end socket
      (set `local.StartLocation` (`SceneComponent.GetSocketLocation` (`self.Mesh`) "FishSocket"))
      ;[0.05098 0.05098 0.05098] End Position Location from where we are looking multiplied by rod distance
      (set `local.EndLocation` (+ (`local.StartLocation`) (* (`KismetMathLibrary.GetForwardVector` (`Controller.GetControlRotation` (`Pawn.GetController` (`self.Instigator`)))) (`self.LineLength`))))
      (bind _tossvelocity (`GameplayStatics.BlueprintSuggestProjectileVelocity` (`local.StartLocation`) (`local.EndLocation`) (`self.LineLength`) 0.0 "DoNotTrace" 10.0))
      (return (`local.StartLocation`) _tossvelocity))
    (:`else`)))

(fn `ClearFishArc`
  (bind _splinemeshes (`self.splineMeshes`))
  (`SplineComponent.ClearSplinePoints` (`self.Spline`) true)
  (for _array_element _splinemeshes
    (`ActorComponent.K2_DestroyComponent` _array_element))
  (`KismetArrayLibrary.Array_Clear` _splinemeshes))

(fn `DestroyBait`
  (bind _bait (`self.Bait`)
    (:`then`
      (`self.K2_DestroyActor` _bait))
    (:`else`)))

(fn `GetBait`
  (returns (`Fishing Bait` :type "/Game/FPSFishing/Blueprints/Fishing/BP_FishingBait_asset Object Reference"))
  (return (`self.Bait`)))

(fn `OnBaitEaten`
  (params (Bait :type "/Game/FPSFishing/Blueprints/Fishing/BP_FishingBait_asset Object Reference") (EatenBy :type "/Game/FPSFishing/Blueprints/Fishing/BP_Fish_asset Object Reference"))
  (`CableComponent.SetAttachEndToComponent` (`self.Cable`) (`/Game/FPSFishing/Blueprints/Fishing/BP_Fish_asset.StaticMesh` EatenBy) "None"))

(fn `PullCable`
  (params (Alpha :type "Float (single-precision)"))
  (locals (AttachedActor :type "Actor Object Reference"))
  (bind _output_get (set `local.AttachedActor` (`CableComponent.GetAttachedActor` (`self.Cable`))))
  (`/Engine/EditorBlueprintResources/StandardMacros.IsValid` _output_get
    (:`Is Valid`
      (`/Engine/EditorBlueprintResources/StandardMacros.IsValid` (`self.GetAttachParentActor` (`local.AttachedActor`))
        (:`Is Not Valid`
          (`self.K2_SetActorLocationAndRotation` (`local.AttachedActor`) (`KismetMathLibrary.VLerp` (`self.K2_GetActorLocation` (`local.AttachedActor`)) (`SceneComponent.GetSocketLocation` (`self.Mesh`) "FishHangingSocket") (`local.Alpha`)) (`KismetMathLibrary.RLerp` (`self.Rot1`) (`self.Rot2`) (`local.Alpha`)) false false))))))

(fn `ResetCable`
  (set `CableComponent.bAttachEnd` false (`self.Cable`))
  (`CableComponent.SetAttachEndTo` (`self.Cable`) null "None" "None")
  ;[0.05098 0.05098 0.05098] Hide Cable
  (`SceneComponent.SetVisibility` (`self.Cable`) false false))

(fn `SetSize`
  (params (Scale :type "Float (double-precision)"))
  (set `CableComponent.CableLength` (* Scale 100.0) (`self.Cable`)))

(fn `Throw Bait`
  (locals (Bait :type "/Game/FPSFishing/Blueprints/Fishing/BP_FishingBait_asset Object Reference"))
  (`/Engine/EditorBlueprintResources/StandardMacros.IsValid` (`self.Bait`)
    (:`Is Valid`
      (bind (_startpos _launchvelocity) (`self.CalcThrowTrajectory`))
      (`/Game/FPSFishing/Blueprints/Fishing/BP_FishingBait_asset.Throw` (`self.Bait`) _launchvelocity))))

(fn `UpdateFishArc`
  (bind _spline (`self.Spline`))
  (bind (_startpos _launchvelocity) (`self.CalcThrowTrajectory`))
  (bind (_outhit _outpathpositions) (`GameplayStatics.Blueprint_PredictProjectilePath_ByTraceChannel` _startpos _launchvelocity true 1.0 "ECC_Visibility" false (`|MakeArray` self :!type "Actor Object Reference") "None" 1.0 15.0 3.0))
  (`self.ClearFishArc`)
  (for (_array_element _array_index) _outpathpositions
    (`SplineComponent.AddSplinePointAtIndex` (`self.Spline`) _array_element _array_index "Local" false))
  (for _index (range (+ (- (`SplineComponent.GetNumberOfSplinePoints` (`self.Spline`)) 2) 1))
    (bind _returnvalue (`AddComponent|NODE_AddSplineMeshComponent-0` :`bManualAttachment` true))
    (bind (_location _tangent) (`SplineComponent.GetLocationAndTangentAtSplinePoint` _spline _index "Local"))
    (bind (_location_2 _tangent_2) (`SplineComponent.GetLocationAndTangentAtSplinePoint` _spline (+ _index 1) "Local"))
    (`SplineMeshComponent.SetStartAndEnd` _returnvalue _location _tangent _location_2 _tangent_2 true)
    (`PrimitiveComponent.SetMaterial` _returnvalue 0 (`self.SplineMat`))
    (`KismetArrayLibrary.Array_Add` (`self.splineMeshes`) _returnvalue))
  (bind (_bblockinghit _binitialoverlap _time _distance _location_3 _impactpoint _normal _impactnormal _physmat _hitactor) (`GameplayStatics.BreakHitResult` _outhit))
  (`/Engine/EditorBlueprintResources/StandardMacros.IsValid` _hitactor
    (:`Is Valid`
      (`MaterialInstanceDynamic.SetVectorParameterValue` (`self.SplineMat`) "Color" (`KismetMathLibrary.SelectColor` (struct :`G` 0.46875 :`B` 0.026692 :`A` 1.0) (struct :`R` 1.0 :`A` 1.0) (`KismetSystemLibrary.IsValid` (`self.GetComponentByClass` _hitactor "/Game/FPSFishing/Blueprints/Fishing/BP_FishableAreaComponent_asset.BP_FishableAreaComponent_asset_C")))))
    (:`Is Not Valid`
      (`MaterialInstanceDynamic.SetVectorParameterValue` (`self.SplineMat`) "Color" (struct :`R` 1.0 :`A` 1.0)))))

(fn `UserConstructionScript`)