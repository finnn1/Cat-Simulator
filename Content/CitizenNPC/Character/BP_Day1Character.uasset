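; BP_Day1Character is a citizen NPC character that walks along the path of a BP_Spline actor found in the level at BeginPlay.
; Each Tick advances a distance counter by Speed until the spline ends, feeding the tangent at that distance into AddMovementInput.
; It steers by direction only, without correcting position onto the spline.
; When the inherited EffectFin event fires, it calls the parent and destroys itself.
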(event `self.ReceiveBeginPlay`
  (`parent.ReceiveBeginPlay`)
  (bind _returnvalue (`GameplayStatics.GetActorOfClass` "/Game/CitizenNPC/Character/BP_Spline.BP_Spline_C"))
  (set `self.Spline` _returnvalue)
  (set `self.SplineLength` 0.0))

(event `self.ReceiveTick`
  (params (DeltaSeconds :type "Float (single-precision)"))
  (bind _spline (`self.Spline`))
  (bind _returnvalue (`SplineComponent.GetSplineLength` (`/Game/CitizenNPC/Character/BP_Spline.Spline` _spline)))
  (`/Engine/EditorBlueprintResources/StandardMacros.IsValid` _spline
    (:`Is Valid`
      (if (not (>= (`self.SplineLength`) _returnvalue))
        (bind _output_get (set `self.SplineLength` (`KismetMathLibrary.FClamp` (+ (* DeltaSeconds (`self.Speed`)) (`self.SplineLength`)) 0.0 _returnvalue)))
        (`self.AddMovementInput` (`KismetMathLibrary.Normal` (`SplineComponent.GetTangentAtDistanceAlongSpline` (`/Game/CitizenNPC/Character/BP_Spline.Spline` (`self.Spline`)) _output_get "World")))))))

(event `self.EffectFin`
  (`parent.EffectFin`)
  (`self.K2_DestroyActor`))

(fn `UserConstructionScript`)