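; An NPC interact component that keeps its pawn wandering around the level.
; From BeginPlay, RandomRoam loops AI MoveTo calls to random reachable points within a radius of the pawn, picking a new point on either success or failure.
; When perception stops sensing the VR pawn, it clears the Interacted flag and sets the NPC's walk speed to a fixed value.
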(event `self.ReceiveBeginPlay`
  (`parent.ReceiveBeginPlay`)
  (`self.Random Roam`))

(event `Random Roam`
  (bind _mypawn (`self.MyPawn`))
  (`|AIMoveTo` _mypawn (`NavigationSystemV1.K2_GetRandomReachablePointInRadius` (`Actor.K2_GetActorLocation` _mypawn) 2500.0 null null) null
    (:`OnSuccess`
      _)
    (:`OnFail`
      _))
  (`self.Random Roam`))

(event `self.OnTargetPerceptionUpdated_Event`
  (params (Actor :type "Actor Object Reference") (Stimulus :type "AIStimulus Structure"))
  (cast `/Game/VRTemplate/Blueprints/S_VRPawnTest` Actor)
  (if (not Stimulus_bSuccessfullySensed)
    (set `self.Interacted` false)
    (set `CharacterMovementComponent.MaxWalkSpeed` 200.0 (`Actor.GetComponentByClass` (`self.MyPawn`) "/Script/Engine.CharacterMovementComponent"))))