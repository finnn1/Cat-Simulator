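; Actor component that handles player interaction for NPC pawns, with dialogue and animation that vary by game day.
; At BeginPlay it caches that day's line and montage from DT_NPC and binds to AI perception.
; Interact stops movement, turns the NPC toward the player, shows the line widget and plays the montage, also completing Quest 2 on Day 1.
; Losing sight of the VR player hides the widget and restores rotation; walk speed restoration is unconnected.
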(event `Interact`
  (params (PlayerLocation :type "Vector Structure"))
  (bind _mypawn (`self.MyPawn`))
  (bind _returnvalue (`Actor.GetComponentByClass` (`self.MyPawn`) "/Script/UMG.WidgetComponent"))
  (bind _ascat_game_instance (cast `CatGameInstance` (`GameplayStatics.GetGameInstance`)))
  (if (== (`CatGameInstance.Day` _ascat_game_instance) 1)
    ;[1 1 1] Stop NPC
    (bind _asvrgame_mode (cast `/Game/VRTemplate/Blueprints/VRGameMode` (`GameplayStatics.GetGameMode`)))
    (set `/Game/VRTemplate/Blueprints/VRGameMode.Quest2Comp` true _asvrgame_mode)
    (`/Game/VRTemplate/Blueprints/VRGameMode.CheckDailyQuest` _asvrgame_mode))
  (set `CharacterMovementComponent.MaxWalkSpeed` 0.0 (`Actor.GetComponentByClass` _mypawn "/Script/Engine.CharacterMovementComponent"))
  (set `self.BeforeRot` (`Actor.K2_GetActorRotation` _mypawn))
  ;[1 1 1] Set Widget
  (`Actor.K2_SetActorRotation` (`self.MyPawn`) (`KismetMathLibrary.FindLookAtRotation` (`Actor.K2_GetActorLocation` (`self.MyPawn`)) PlayerLocation) false)
  (bind _aswbp_interact (cast `/Game/JHR/WBP_Interact` (`WidgetComponent.GetWidget` _returnvalue)))
  (set `/Game/JHR/WBP_Interact.Line` (`self.TodayLine`) _aswbp_interact)
  (`WidgetComponent.SetTintColorAndOpacity` _returnvalue (struct :`R` 1.0 :`G` 1.0 :`B` 1.0 :`A` 1.0))
  (bind _ascharacter (cast `Character` (`self.MyPawn`)))
  (`Character.PlayAnimMontage` _ascharacter (`self.DailyAnim`) 1.0 "None"))

(event `self.ReceiveBeginPlay`
  ;[1 1 1] Comment
  (bind _aspawn (cast `Pawn` (`self.GetOwner`)))
  (set `self.MyPawn` _aspawn)
  ;[1 1 1] Comment
  (bind _ascat_game_instance (cast `CatGameInstance` (`GameplayStatics.GetGameInstance`)))
  (bind _returnvalue (`|GetDataTableRow` "/Game/JHR/Data/DT_NPC.DT_NPC" (`self.Index`))
    (:`then`
      (bind _returnvalue_2 (- (`CatGameInstance.Day` _ascat_game_instance) 1))
      (set `self.TodayLine` (`|GetArrayItem` (`.Line_5_D05E98D2451529E118D6F48AD91418C7` (break `/Game/JHR/Data/S_NPC` _returnvalue)) _returnvalue_2))
      (set `self.DailyAnim` (`|GetArrayItem` (`.DailyAnimations_9_1B5C02C648C288E70C528898E711CE7A` (break `/Game/JHR/Data/S_NPC` _returnvalue)) _returnvalue_2))
      (add `AIPerceptionComponent.OnTargetPerceptionUpdated` (`Actor.GetComponentByClass` (`self.MyPawn`) "/Script/AIModule.AIPerceptionComponent") (delegate `OnTargetPerceptionUpdated_Event`)))))

(event `OnTargetPerceptionUpdated_Event`
  (params (Actor :type "Actor Object Reference") (Stimulus :type "AIStimulus Structure"))
  (bind _mypawn (`self.MyPawn`))
  (cast `/Game/VRTemplate/Blueprints/S_VRPawnTest` Actor)
  (if Stimulus_bSuccessfullySensed
    (set `self.Interacted` true)
    (else
      (set `self.Interacted` false)
      ;[1 1 1] Set Widget Component
      (`WidgetComponent.SetTintColorAndOpacity` :`self` (`Actor.GetComponentByClass` _mypawn "/Script/UMG.WidgetComponent"))
      (`Actor.K2_SetActorRotation` _mypawn (`self.BeforeRot`) false))))