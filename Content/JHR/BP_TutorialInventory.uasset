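; BP_TutorialInventory is a tutorial indicator that marks the inventory step as finished once the VR player holds an item.
; Every Tick it looks up S_VRPawnTest and checks the left and right hand items in its BPInventorySystem.
; If either is valid, it sets the Cube's material to Mat_TutoFin, reapplying it each frame.
; The BP_NPC cached on BeginPlay feeds only disconnected logic, as does a similar Menu check.
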(event `self.ReceiveBeginPlay`
  (bind _returnvalue (`GameplayStatics.GetActorOfClass` "/Game/JHR/BP_NPC.BP_NPC_C"))
  (set `self.As BP NPC` _returnvalue))

(event `self.ReceiveActorBeginOverlap`
  (params (OtherActor :type "Actor Object Reference")))

(event `self.ReceiveTick`
  (params (DeltaSeconds :type "Float (single-precision)"))
  (`|ExecutionSequence`
    (:`then_0`
      (bind _returnvalue (`GameplayStatics.GetActorOfClass` "/Game/VRTemplate/Blueprints/S_VRPawnTest.S_VRPawnTest_C"))
      (`/Engine/EditorBlueprintResources/StandardMacros.IsValid` _returnvalue
        (:`Is Valid`
          (bind _bp_inventorysystem (`/Game/VRTemplate/Blueprints/S_VRPawnTest.BP_InventorySystem` _returnvalue))
          (if (or (`KismetSystemLibrary.IsValid` (`InventorySystem.ItemInLeftHand` _bp_inventorysystem)) (`KismetSystemLibrary.IsValid` (`InventorySystem.ItemInRightHand` _bp_inventorysystem)))
            (`PrimitiveComponent.SetMaterial` (`self.Cube`) 0 "/Game/JHR/Mat_TutoFin.Mat_TutoFin")))))))

(fn `UserConstructionScript`)