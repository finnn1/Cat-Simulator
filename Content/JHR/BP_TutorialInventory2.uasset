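; Tutorial marker actor, apparently for an inventory step, whose Cube switches to a completion material when the Menu actor's Tu flag is set.
; Tick looks up the Menu actor every frame and reapplies the material while the flag holds, with both Sequence outputs running the same check.
; BeginPlay caches BP_NPC, but the NPC-interaction and VR-pawn held-item checks are disconnected and never run.
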(event `self.ReceiveBeginPlay`
  (bind _returnvalue (`GameplayStatics.GetActorOfClass` "/Game/JHR/BP_NPC.BP_NPC_C"))
  (set `self.As BP NPC` _returnvalue))

(event `self.ReceiveActorBeginOverlap`
  (params (OtherActor :type "Actor Object Reference")))

(event `self.ReceiveTick`
  (params (DeltaSeconds :type "Float (single-precision)"))
  (`|ExecutionSequence`
    (:`then_0`
      _)
    (:`then_1`
      _))
  (bind _returnvalue (`GameplayStatics.GetActorOfClass` "/Game/VRTemplate/Blueprints/Menu.Menu_C"))
  (`/Engine/EditorBlueprintResources/StandardMacros.IsValid` _returnvalue
    (:`Is Valid`
      (if (`/Game/VRTemplate/Blueprints/Menu.bTu` _returnvalue)
        (`PrimitiveComponent.SetMaterial` (`self.Cube`) 0 "/Game/JHR/Mat_TutoFin.Mat_TutoFin")))))

(fn `UserConstructionScript`)