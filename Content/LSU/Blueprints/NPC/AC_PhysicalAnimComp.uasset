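; Actor component that gives a character a physics-driven reaction to an impulse, going by its setup in the NPC folder.
; BeginPlay adds a PhysicalAnimationComponent bound to the owning Character's mesh and caches mesh references.
; TogglePhysicalAnimation simulates physics below the pelvis, applies an AttackPower-scaled impulse, then after a delay calls EffectFin on BP_Character.
; The physical animation profile nodes are disconnected, so the reaction is plain ragdoll simulation.
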(event `self.ReceiveBeginPlay`
  (`|ExecutionSequence`
    (:`then_0`
      (bind _returnvalue (`|AddComponentByClass` (`self.GetOwner`) "/Script/Engine.PhysicalAnimationComponent"))
      (bind _output_get (set `self.PhysicalAnimationComponent` _returnvalue))
      (bind _ascharacter (cast `Character` (`self.GetOwner`)))
      (bind _mesh (`Character.Mesh` _ascharacter))
      (`PhysicalAnimationComponent.SetSkeletalMeshComponent` _output_get _mesh)
      (set `self.Mesh` _mesh)
      (set `self.Capsule Component` (`Character.CapsuleComponent` _ascharacter)))
    (:`then_1`
      (set `self.SK_Arr` (`Actor.K2_GetComponentsByClass` (`self.GetOwner`) "/Script/Engine.SkeletalMeshComponent")))))

(event `TogglePhysicalAnimation`
  (params (ImpulseVec :type "Vector Structure"))
  (bind _mesh (`self.Mesh`))
  (bind _mesh_2 (`self.Mesh`))
  (`PrimitiveComponent.SetSimulatePhysics` (`self.Mesh`) true)
  (`SkeletalMeshComponent.SetAllBodiesBelowSimulatePhysics` _mesh "pelvis" true false)
  (`SkeletalMeshComponent.SetAllBodiesBelowPhysicsBlendWeight` _mesh "pelvis" 1.0 false true)
  (`PrimitiveComponent.AddImpulse` _mesh_2 (* ImpulseVec (`self.AttackPower`)) "None" true)
  (`KismetSystemLibrary.Delay` 5.0)
  (bind _asbp_character (cast `/Game/CitizenNPC/Character/Blueprints/BP_Character` (`self.GetOwner` _mesh_2)))
  (`/Game/CitizenNPC/Character/Blueprints/BP_Character.EffectFin` _asbp_character))