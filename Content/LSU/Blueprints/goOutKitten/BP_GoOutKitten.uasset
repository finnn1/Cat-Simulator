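; BP_GoOutKitten is an actor that travels along a BP_SplineKitten path and can be fed by the player.
; On BeginPlay a timeline moves it along the spline with a random horizontal offset, rotated to face the spline tangent.
; When interacted with using a food item on its owning BP_Kitten's food list, it refills that kitten's food, reveals its mesh, restarts its food timer and hides itself.
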(event `self.ReceiveBeginPlay`
  (bind _randomoffset (`self.RandomOffset`))
  (bind _spline (`/Game/LSU/Blueprints/goOutKitten/BP_SplineKitten.Spline` (`self.kittenSpline`)))
  (bind _returnvalue (`GameplayStatics.GetActorOfClass` "/Game/LSU/Blueprints/goOutKitten/BP_SplineKitten.BP_SplineKitten_C"))
  (bind _output_get (set `self.kittenSpline` _returnvalue))
  (`self.K2_SetActorLocation` (`SplineComponent.GetLocationAtDistanceAlongSpline` (`/Game/LSU/Blueprints/goOutKitten/BP_SplineKitten.Spline` _output_get) 0.0 "World"))
  (set `self.RandomOffset` (`KismetMathLibrary.RandomFloatInRange` -100.0 100.0))
  (bind (_direction _newtrack_0) (`Timeline|Timeline`)
    (:`Update`
      (bind _returnvalue_2 (* _newtrack_0 (`SplineComponent.GetSplineLength` _spline)))
      (`self.K2_SetActorLocation` (+ (`SplineComponent.GetLocationAtDistanceAlongSpline` _spline _returnvalue_2 "World") (`KismetMathLibrary.MakeVector` _randomoffset _randomoffset)))
      (`self.K2_SetActorRotation` (`KismetMathLibrary.Conv_VectorToRotator` (`SplineComponent.GetTangentAtDistanceAlongSpline` _spline _returnvalue_2 "World"))))))

(event `/Game/LSU/Blueprints/Kitten/BPI_InteractPawn.InteractFromName`
  (params (FoodItem :type "/Game/LCU/Item/BP_FoodItem Object Reference"))
  (bind (_asbp_kitten _bsuccess) (cast `/Game/LSU/Blueprints/Kitten/BP_Kitten` (`self.MyOwner`) :!pure true))
  (bind (_itemid_datatable _itemid_rowname) (break `DataTableRowHandle` (`UItemDataComponent.ItemID` (`UItem.ItemDataComponent` FoodItem))))
  (if _bsuccess
    (if (!= (`KismetArrayLibrary.Array_Find` (`/Game/LSU/Blueprints/Kitten/BP_Kitten.FoodList` _asbp_kitten) _itemid_rowname) -1)
      (set `Kitten.KittenCurrentFood` 50.0 _asbp_kitten)
      (`SceneComponent.SetVisibility` (`Kitten.KittenMesh` _asbp_kitten) true false)
      (`Kitten.SetKittenFoodTimer` _asbp_kitten)
      (`self.SetActorHiddenInGame` true))))

(fn `UserConstructionScript`)