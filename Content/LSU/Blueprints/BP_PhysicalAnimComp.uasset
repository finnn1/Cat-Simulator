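; Actor component that adds physical animation support to BP_eonNPC owners, enabling partial physics blending on their skeletal mesh.
; On BeginPlay it creates a PhysicalAnimationComponent on the owner, binds it to the NPC's mesh and caches that mesh.
; TogglePhysicalAnimation only switches on simulation for bodies below the pelvis at a partial blend weight, with no off path.
; The hit-reaction profile and impulse nodes are disconnected.
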(event `self.ReceiveBeginPlay`
  (bind _returnvalue (`|AddComponentByClass` (`self.GetOwner`) "/Script/Engine.PhysicalAnimationComponent"))
  (bind _output_get (set `self.PhysicalAnimationComponent` _returnvalue))
  (bind _asbp_eon_npc (cast `/Game/LSU/Blueprints/BP_eonNPC` (`self.GetOwner`)))
  (bind _mesh (`Character.Mesh` _asbp_eon_npc))
  (`PhysicalAnimationComponent.SetSkeletalMeshComponent` _output_get _mesh)
  (set `self.Mesh` _mesh))

(event `TogglePhysicalAnimation`
  (`SkeletalMeshComponent.SetAllBodiesBelowSimulatePhysics` (`self.Mesh`) "pelvis" true false)
  (`SkeletalMeshComponent.SetAllBodiesBelowPhysicsBlendWeight` (`self.Mesh`) "pelvis" 0.6 false true))