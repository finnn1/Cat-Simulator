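; Black kitten Blueprint that decides how much hunger value a consumed item gives this kitten.
; TakeFood flags the item as used and looks up its data table row through the item's ItemDataComponent.
; If the row has a HUNGER property, ItemPoint takes that value for items in FoodList and zero for any other.
; The event graph and construction script hold no active logic.
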(event `self.ReceiveBeginPlay`)

(event `self.ReceiveTick`
  (params (DeltaSeconds :type "Float (single-precision)")))

(fn `TakeFood`
  (params (ConsumeItem :type "/Game/LCU/Item/BP_FoodItem Object Reference"))
  (bind (_itemid_datatable _itemid_rowname) (break `DataTableRowHandle` (`UItemDataComponent.ItemID` (`UItem.ItemDataComponent` ConsumeItem))))
  (set `self.UseItem` true)
  (bind _returnvalue (`|GetDataTableRow` _itemid_datatable _itemid_rowname)
    (:`then`
      (bind (_value _returnvalue_2) (`BlueprintMapLibrary.Map_Find` (`.ItemProperty` (break `ItemStruct` _returnvalue)) "HUNGER"))
      (if _returnvalue_2
        (if (!= (`KismetArrayLibrary.Array_Find` (`self.FoodList`) _itemid_rowname) -1)
          (set `self.ItemPoint` _value)
          (else
            (set `self.ItemPoint` 0.0)))))))

(fn `UserConstructionScript`)