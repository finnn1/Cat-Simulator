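; BP_Kitten_Black is the black kitten variant of a parent kitten Blueprint, scoring the food items given to it.
; Its interact event simply forwards the food item to the parent implementation.
; TakeFood flags the item as used and looks up its row name in the VR game mode's BlackItem list.
; A match sets ItemPoint to the item's FullFood value, while any other item yields zero.
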(event `self.ReceiveBeginPlay`)

(event `Key|B`
  (params (Key :type "Key Structure")))

(event `self.ReceiveTick`
  (params (DeltaSeconds :type "Float (single-precision)")))

(event `/Game/LSU/Blueprints/BPI_InteractPawn.InteractFromName`
  (params (FoodItem :type "/Game/LCU/Item/BP_FoodItem Object Reference"))
  (`parent.InteractFromName` FoodItem))

(fn `TakeFood`
  (params (ConsumeItem :type "/Game/LCU/Item/BP_FoodItem Object Reference"))
  (bind (_foodattributes_foodproperties _foodattributes_hp _foodattributes_fullfood) (break `FoodAttributes` (`UFoodItem.FoodAttributes` ConsumeItem)))
  (bind (_itemid_datatable _itemid_rowname) (break `DataTableRowHandle` (`UItemDataComponent.ItemID` (`UItem.ItemDataComponent` ConsumeItem))))
  (set `self.UseItem` true)
  (bind _asvrgame_mode (cast `/Game/VRTemplate/Blueprints/VRGameMode` (`GameplayStatics.GetGameMode`)))
  (if (!= (`KismetArrayLibrary.Array_Find` (`/Game/VRTemplate/Blueprints/VRGameMode.BlackItem` _asvrgame_mode) _itemid_rowname) -1)
    (set `self.ItemPoint` _foodattributes_fullfood)
    (else
      (set `self.ItemPoint` 0.0))))

(fn `UserConstructionScript`)