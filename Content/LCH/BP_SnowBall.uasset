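; BP_SnowBall is a grabbable snowball that bursts on hard impacts with pawns and knocks characters over.
; Its sphere collision hit event ignores the first player's character, non-pawn object types and hits while the GrabComponent holds it.
; When the impulse exceeds ExplosionPowerLimit, it spawns a Niagara explosion and destroys itself.
; A struck BP_Character first loses movement and has physical animation toggled with the reversed impulse.
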(event `self.SphereColl.OnComponentHit`
  (params (HitComponent :type "PrimitiveComponent Object Reference") (OtherActor :type "Actor Object Reference") (OtherComp :type "PrimitiveComponent Object Reference") (NormalImpulse :type "Vector Structure") (Hit :type "HitResult Structure (by ref)"))
  (bind _asbp_character (cast `/Game/CitizenNPC/Character/Blueprints/BP_Character` OtherActor :!pure true))
  (if (and (!= OtherActor (`GameplayStatics.GetPlayerCharacter` 0)) (not (`/Game/VRTemplate/Blueprints/GrabComponent.bIsHeld` (`self.GrabComponent`))) (== (`|GetEnumeratorName` (`PrimitiveComponent.GetCollisionObjectType` OtherComp)) "ECC_Pawn"))
    (if (> (`KismetMathLibrary.VSize` NormalImpulse) (`self.ExplosionPowerLimit`))
      (`NiagaraFunctionLibrary.SpawnSystemAtLocation` "/Game/LCH/NS_SnowBallExplosion.NS_SnowBallExplosion" (`.ImpactPoint` (`GameplayStatics.BreakHitResult` Hit)))
      (`/Engine/EditorBlueprintResources/StandardMacros.IsValid` _asbp_character
        (:`Is Valid`
          (`CharacterMovementComponent.DisableMovement` (`Character.CharacterMovement` _asbp_character))
          (`/Game/LSU/Blueprints/NPC/AC_PhysicalAnimComp.TogglePhysicalAnimation` (`/Game/CitizenNPC/Character/Blueprints/BP_Character.AC_PhysicalAnimComp` _asbp_character) (* NormalImpulse -1.0)))
        (:`Is Not Valid`
          _))
      (`self.K2_DestroyActor`))))

(fn `UserConstructionScript`)