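; BP_BasketBallHoop is a basketball hoop that counts scored balls and displays the total.
; When a BP_BasketBall stops overlapping the score box, Score increments and UpdateScore writes it to ScoreText.
; A separate detection box stores the entering ball in DetectedBall and clears it when that ball exits, but scoring never checks this reference, so exit direction and prior detection are ignored.
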(event `self.BallDetectBoxColl.OnComponentBeginOverlap`
  (params (OverlappedComponent :type "PrimitiveComponent Object Reference") (OtherActor :type "Actor Object Reference") (OtherComp :type "PrimitiveComponent Object Reference") (OtherBodyIndex :type Integer) (bFromSweep :type Boolean) (SweepResult :type "HitResult Structure (by ref)"))
  (bind _asbp_basket_ball (cast `/Game/LCH/BP_BasketBall` OtherActor))
  (set `self.DetectedBall` _asbp_basket_ball))

(event `self.BallDetectBoxColl.OnComponentEndOverlap`
  (params (OverlappedComponent :type "PrimitiveComponent Object Reference") (OtherActor :type "Actor Object Reference") (OtherComp :type "PrimitiveComponent Object Reference") (OtherBodyIndex :type Integer))
  (bind _asbp_basket_ball (cast `/Game/LCH/BP_BasketBall` OtherActor))
  (if (== _asbp_basket_ball (`self.DetectedBall`))
    (set `self.DetectedBall` null)))

(event `self.ScoreBoxColl.OnComponentEndOverlap`
  (params (OverlappedComponent :type "PrimitiveComponent Object Reference") (OtherActor :type "Actor Object Reference") (OtherComp :type "PrimitiveComponent Object Reference") (OtherBodyIndex :type Integer))
  (if (`GameplayStatics.ObjectIsA` OtherActor "/Game/LCH/BP_BasketBall.BP_BasketBall_C")
    (bind _output_get (set `self.Score` (+ (`self.Score`) 1)))
    (`self.UpdateScore` _output_get)))

(event `UpdateScore`
  (params (NewScore :type Integer64))
  (`TextRenderComponent.K2_SetText` (`self.ScoreText`) (`KismetTextLibrary.Conv_Int64ToText` NewScore)))

(fn `UserConstructionScript`)